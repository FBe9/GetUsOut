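; VR lever actor with four independent levers that pitch to follow the motion controller holding them.
; Each GrabComponent stores the grabbing controller and starts a fast looping timer by function name for its own UpdateRotation function.
; Those functions add the hand's local Y offset from the grab point to their Scene component's pitch, clamped symmetrically.
; Dropping, or any end overlap on the lever's capsule, clears that timer.
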(event `self.GrabComponent3.OnGrabbed`
  (params (`Motion Controller` :type "MotionControllerComponent Object Reference"))
  ;[1 1 1] Al agarrar la palanca hace que se mueva junto con la mano
  (set `self.Motion Controller` `Motion Controller`)
  (bind _returnvalue (`KismetSystemLibrary.K2_SetTimer` null "UpdateRotation_3" 0.01 true))
  (set `self.Timer3` _returnvalue))

(event `self.GrabComponent3.OnDropped`
  ;[1 1 1] Al agarrar la palanca hace que se mueva junto con la mano
  (`KismetSystemLibrary.K2_ClearAndInvalidateTimerHandle` (`self.Timer3`)))

(event `self.GrabComponent2.OnGrabbed`
  (params (`Motion Controller` :type "MotionControllerComponent Object Reference"))
  ;[1 1 1] Al agarrar la palanca hace que se mueva junto con la mano
  (set `self.Motion Controller_0` `Motion Controller`)
  (bind _returnvalue (`KismetSystemLibrary.K2_SetTimer` null "UpdateRotation_2" 0.01 true))
  (set `self.Timer2` _returnvalue))

(event `self.GrabComponent2.OnDropped`
  ;[1 1 1] Al agarrar la palanca hace que se mueva junto con la mano
  (`KismetSystemLibrary.K2_ClearAndInvalidateTimerHandle` (`self.Timer2`)))

(event `self.GrabComponent.OnGrabbed`
  (params (`Motion Controller` :type "MotionControllerComponent Object Reference"))
  ;[1 1 1] Al agarrar la palanca hace que se mueva junto con la mano
  (set `self.Motion Controller_1` `Motion Controller`)
  (bind _returnvalue (`KismetSystemLibrary.K2_SetTimer` null "UpdateRotation" 0.01 true))
  (set `self.Timer` _returnvalue))

(event `self.GrabComponent.OnDropped`
  ;[1 1 1] Al agarrar la palanca hace que se mueva junto con la mano
  (`KismetSystemLibrary.K2_ClearAndInvalidateTimerHandle` (`self.Timer`)))

(event `self.GrabComponent1.OnGrabbed`
  (params (`Motion Controller` :type "MotionControllerComponent Object Reference"))
  ;[1 1 1] Al agarrar la palanca hace que se mueva junto con la mano
  (set `self.Motion Controller_2` `Motion Controller`)
  (bind _returnvalue (`KismetSystemLibrary.K2_SetTimer` null "UpdateRotation_1" 0.01 true))
  (set `self.Timer1` _returnvalue))

(event `self.GrabComponent1.OnDropped`
  ;[1 1 1] Al agarrar la palanca hace que se mueva junto con la mano
  (`KismetSystemLibrary.K2_ClearAndInvalidateTimerHandle` (`self.Timer1`)))

(event `self.Capsule3.OnComponentEndOverlap`
  (params (OverlappedComponent :type "PrimitiveComponent Object Reference") (OtherActor :type "Actor Object Reference") (OtherComp :type "PrimitiveComponent Object Reference") (OtherBodyIndex :type Integer))
  ;[1 1 1] Al alejarse la mano de la caja de colisión de la cápsula deshabilita el timer
  (`KismetSystemLibrary.K2_ClearAndInvalidateTimerHandle` (`self.Timer3`)))

(event `self.Capsule2.OnComponentEndOverlap`
  (params (OverlappedComponent :type "PrimitiveComponent Object Reference") (OtherActor :type "Actor Object Reference") (OtherComp :type "PrimitiveComponent Object Reference") (OtherBodyIndex :type Integer))
  ;[1 1 1] Al alejarse la mano de la caja de colisión de la cápsula deshabilita el timer
  (`KismetSystemLibrary.K2_ClearAndInvalidateTimerHandle` (`self.Timer2`)))

(event `self.Capsule.OnComponentEndOverlap`
  (params (OverlappedComponent :type "PrimitiveComponent Object Reference") (OtherActor :type "Actor Object Reference") (OtherComp :type "PrimitiveComponent Object Reference") (OtherBodyIndex :type Integer))
  ;[1 1 1] Al alejarse la mano de la caja de colisión de la cápsula deshabilita el timer
  (`KismetSystemLibrary.K2_ClearAndInvalidateTimerHandle` (`self.Timer`)))

(event `self.Capsule1.OnComponentEndOverlap`
  (params (OverlappedComponent :type "PrimitiveComponent Object Reference") (OtherActor :type "Actor Object Reference") (OtherComp :type "PrimitiveComponent Object Reference") (OtherBodyIndex :type Integer))
  ;[1 1 1] Al alejarse la mano de la caja de colisión de la cápsula deshabilita el timer
  (`KismetSystemLibrary.K2_ClearAndInvalidateTimerHandle` (`self.Timer1`)))

(fn `UpdateRotation`
  (bind _scene (`self.Scene`))
  (bind _grabcomponent (`self.GrabComponent`))
  (bind (_relativerotation_roll _relativerotation_pitch _relativerotation_yaw) (`KismetMathLibrary.BreakRotator` (`SceneComponent.RelativeRotation` _scene)))
  (bind _returnvalue_location (`KismetMathLibrary.BreakTransform` (`KismetMathLibrary.MakeRelativeTransform` (`SceneComponent.K2_GetComponentToWorld` (`self.Motion Controller_1`)) (`SceneComponent.K2_GetComponentToWorld` _grabcomponent))))
  (bind (_returnvalue_x _returnvalue_y) (`KismetMathLibrary.BreakVector` (- _returnvalue_location (`SceneComponent.RelativeLocation` _grabcomponent))))
  (`SceneComponent.K2_SetRelativeRotation` _scene (`KismetMathLibrary.MakeRotator` _relativerotation_roll (`KismetMathLibrary.FClamp` (+ _relativerotation_pitch _returnvalue_y) -40.0 40.0) _relativerotation_yaw) false false))

(fn `UpdateRotation_1`
  (bind _scene1 (`self.Scene1`))
  (bind _grabcomponent1 (`self.GrabComponent1`))
  (bind (_relativerotation_roll _relativerotation_pitch _relativerotation_yaw) (`KismetMathLibrary.BreakRotator` (`SceneComponent.RelativeRotation` _scene1)))
  (bind _returnvalue_location (`KismetMathLibrary.BreakTransform` (`KismetMathLibrary.MakeRelativeTransform` (`SceneComponent.K2_GetComponentToWorld` (`self.Motion Controller_2`)) (`SceneComponent.K2_GetComponentToWorld` _grabcomponent1))))
  (bind (_returnvalue_x _returnvalue_y) (`KismetMathLibrary.BreakVector` (- _returnvalue_location (`SceneComponent.RelativeLocation` _grabcomponent1))))
  (`SceneComponent.K2_SetRelativeRotation` _scene1 (`KismetMathLibrary.MakeRotator` _relativerotation_roll (`KismetMathLibrary.FClamp` (+ _relativerotation_pitch _returnvalue_y) -40.0 40.0) _relativerotation_yaw) false false))

(fn `UpdateRotation_2`
  (bind _scene2 (`self.Scene2`))
  (bind _grabcomponent2 (`self.GrabComponent2`))
  (bind (_relativerotation_roll _relativerotation_pitch _relativerotation_yaw) (`KismetMathLibrary.BreakRotator` (`SceneComponent.RelativeRotation` _scene2)))
  (bind _returnvalue_location (`KismetMathLibrary.BreakTransform` (`KismetMathLibrary.MakeRelativeTransform` (`SceneComponent.K2_GetComponentToWorld` (`self.Motion Controller_0`)) (`SceneComponent.K2_GetComponentToWorld` _grabcomponent2))))
  (bind (_returnvalue_x _returnvalue_y) (`KismetMathLibrary.BreakVector` (- _returnvalue_location (`SceneComponent.RelativeLocation` _grabcomponent2))))
  (`SceneComponent.K2_SetRelativeRotation` _scene2 (`KismetMathLibrary.MakeRotator` _relativerotation_roll (`KismetMathLibrary.FClamp` (+ _relativerotation_pitch _returnvalue_y) -40.0 40.0) _relativerotation_yaw) false false))

(fn `UpdateRotation_3`
  (bind _grabcomponent3 (`self.GrabComponent3`))
  (bind _scene3 (`self.Scene3`))
  (bind (_relativerotation_roll _relativerotation_pitch _relativerotation_yaw) (`KismetMathLibrary.BreakRotator` (`SceneComponent.RelativeRotation` _scene3)))
  (bind _returnvalue_location (`KismetMathLibrary.BreakTransform` (`KismetMathLibrary.MakeRelativeTransform` (`SceneComponent.K2_GetComponentToWorld` (`self.Motion Controller`)) (`SceneComponent.K2_GetComponentToWorld` _grabcomponent3))))
  (bind (_returnvalue_x _returnvalue_y) (`KismetMathLibrary.BreakVector` (- _returnvalue_location (`SceneComponent.RelativeLocation` _grabcomponent3))))
  (`SceneComponent.K2_SetRelativeRotation` _scene3 (`KismetMathLibrary.MakeRotator` _relativerotation_roll (`KismetMathLibrary.FClamp` (+ _relativerotation_pitch _returnvalue_y) -40.0 40.0) _relativerotation_yaw) false false))

(fn `UserConstructionScript`)