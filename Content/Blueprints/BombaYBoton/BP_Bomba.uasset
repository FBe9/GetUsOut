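; BP_Bomba is a defusable bomb actor that counts down from BeginPlay through a one-second function timer calling BombTimer.
; Error plays a ping and cuts five from the remaining time, while Correct tallies successes and disarms the bomb at five by clearing Looping, the flag gating countdown and penalties.
; At zero, Explosion prints a death message, destroys the actor, then still calls a sound node with no sound set and TimerStart.
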(event `self.ReceiveBeginPlay`
  (`self.TimerStart`))

(event `TimerStart`
  (bind _returnvalue (`KismetSystemLibrary.K2_SetTimer` null "BombTimer" 1.0 (`self.Looping`)))
  (set `self.Timer` _returnvalue))

(fn `BombTimer`
  ;[1 1 1] Temporizador - Game Mode
  (if (`self.Looping`)
    (if (>= (`self.TimerBomb`) 0)
      (`/Engine/EditorBlueprintResources/StandardMacros.DecrementInt` (`self.TimerBomb`)
        (:`  `
          (bind _output_get (set `self.TimerBomb` (`self.TimerBomb`)))
          (if (<= _output_get 0)
            (`self.Explosion`)))))))

(fn `Correct`
  (bind _correctnumber (`self.CorrectNumber`))
  (`/Engine/EditorBlueprintResources/StandardMacros.IncrementInt` _correctnumber
    (:`  `
      (if (>= _correctnumber 5)
        (`KismetSystemLibrary.PrintString` "Desactivado")
        (set `self.Looping` false)))))

(fn `Error`
  (if (`self.Looping`)
    (bind _output_get (set `self.TimerBomb` (- (`self.TimerBomb`) 5)))
    (`GameplayStatics.PlaySoundAtLocation` "/Engine/EngineSounds/1kSineTonePing.1kSineTonePing" (`self.K2_GetActorLocation`) (struct) 1.0 1.0 0.0 null null null null)
    (if (<= _output_get 0)
      (`self.Explosion`))))

(fn `Explosion`
  (`KismetSystemLibrary.PrintString` "LUL U DEAD")
  (`self.K2_DestroyActor`)
  (`GameplayStatics.PlaySoundAtLocation` null (`self.K2_GetActorLocation`) (struct) 1.0 1.0 0.0 null null null null)
  (`self.TimerStart`))

(fn `UserConstructionScript`)