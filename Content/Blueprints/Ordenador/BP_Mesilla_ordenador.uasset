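; Nightstand in the computer ("Ordenador") area whose top drawer opens to make a puzzle cube and battery ("pila") available.
; BeginPlay finds both BP_Cubo_Puzle actors by tag and array index, then sets their meshes to PhysicsOnly so queries ignore them.
; AbrirCajon slides the drawer along local X with MoveComponentTo, then restores QueryAndPhysics collision on both items.
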(event `AbrirCajon`
  (bind _v001_mesilla_cajon_cajon_arriba (`self.v001_Mesilla_Cajon_Cajon_Arriba`))
  (bind (_relativelocation_x _relativelocation_y _relativelocation_z) (`KismetMathLibrary.BreakVector` (`SceneComponent.RelativeLocation` _v001_mesilla_cajon_cajon_arriba)))
  (`KismetSystemLibrary.MoveComponentTo` _v001_mesilla_cajon_cajon_arriba (`KismetMathLibrary.MakeVector` 45.0 _relativelocation_y _relativelocation_z) (struct) false false 1.0)
  (`KismetSystemLibrary.PrintString` "movido")
  (`PrimitiveComponent.SetCollisionEnabled` (`/Game/Blueprints/Caja_Puzle/BP_Cubo_Puzle.StaticMesh` (`self.BP_Cubo`)) "QueryAndPhysics")
  (`PrimitiveComponent.SetCollisionEnabled` (`/Game/Blueprints/Caja_Puzle/BP_Cubo_Puzle.StaticMesh` (`self.BP_Pila`)) "QueryAndPhysics"))

(event `self.ReceiveBeginPlay`
  (bind _outactors (`GameplayStatics.GetAllActorsOfClassWithTag` "/Game/Blueprints/Caja_Puzle/BP_Cubo_Puzle.BP_Cubo_Puzle_C" "1"))
  (bind _output_get (set `self.BP_Cubo` (`|GetArrayItem` _outactors 2)))
  (`PrimitiveComponent.SetCollisionEnabled` (`/Game/Blueprints/Caja_Puzle/BP_Cubo_Puzle.StaticMesh` _output_get) "PhysicsOnly")
  (bind _outactors_2 (`GameplayStatics.GetAllActorsOfClassWithTag` "/Game/Blueprints/Caja_Puzle/BP_Cubo_Puzle.BP_Cubo_Puzle_C" "pila1"))
  (bind _output_get_2 (set `self.BP_Pila` (`|GetArrayItem` _outactors_2)))
  (`PrimitiveComponent.SetCollisionEnabled` (`/Game/Blueprints/Caja_Puzle/BP_Cubo_Puzle.StaticMesh` _output_get_2) "PhysicsOnly"))

(fn `UserConstructionScript`)