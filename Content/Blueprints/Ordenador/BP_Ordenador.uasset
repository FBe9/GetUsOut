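; Computer keypad puzzle: entering the correct four-digit code opens the drawer of BP_Mesilla_ordenador.
; Box overlaps sink and raise button meshes; digit boxes pass their component tag as the number, tracked by Contador, while delete clears the previous slot.
; Multicast-named events update the WID_PantallaOrdenador screen; OK compares the code with CodigoCorrecto, showing green OPEN or flashing red before restoring per-digit colours.
; A separate event feeds the post-it widget.
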(event `self.Box_1.OnComponentEndOverlap`
  (params (OverlappedComponent :type "PrimitiveComponent Object Reference") (OtherActor :type "Actor Object Reference") (OtherComp :type "PrimitiveComponent Object Reference") (OtherBodyIndex :type Integer))
  (bind _v001_ordenador_posicionado_boton4_1_ (`self.v001_Ordenador_Posicionado_Boton4(1)`))
  (bind (_relativelocation_x _relativelocation_y _relativelocation_z) (`KismetMathLibrary.BreakVector` (`SceneComponent.RelativeLocation` _v001_ordenador_posicionado_boton4_1_)))
  ;[1 0.5511 0] Retorna a la posicion inical los botones cuando el objeto deja de estar encima
  (`KismetSystemLibrary.MoveComponentTo` _v001_ordenador_posicionado_boton4_1_ (`KismetMathLibrary.MakeVector` 0.0 0.0 (`KismetMathLibrary.FClamp` (+ _relativelocation_z 0.2) -0.4 0.0)) (struct) false false (`self.MovementSeconds`)))

(event `self.Box_4.OnComponentBeginOverlap`
  (params (OverlappedComponent :type "PrimitiveComponent Object Reference") (OtherActor :type "Actor Object Reference") (OtherComp :type "PrimitiveComponent Object Reference") (OtherBodyIndex :type Integer) (bFromSweep :type Boolean) (SweepResult :type "HitResult Structure (by ref)"))
  (bind _v001_ordenador_posicionado_boton7_4_ (`self.v001_Ordenador_Posicionado_Boton7(4)`))
  (bind (_relativelocation_x _relativelocation_y _relativelocation_z) (`KismetMathLibrary.BreakVector` (`SceneComponent.RelativeLocation` _v001_ordenador_posicionado_boton7_4_)))
  ;[1 0.5511 0] Cuando se pulse un botón lo mueve se llama al metodo ButtonAnimation pasandole el boton y el numero que tiene
  (`KismetSystemLibrary.MoveComponentTo` _v001_ordenador_posicionado_boton7_4_ (`KismetMathLibrary.MakeVector` 0.0 0.0 (`KismetMathLibrary.FClamp` (- _relativelocation_z 0.2) -0.4 0.0)) (struct) false false (`self.MovementSeconds`))
  (`/Engine/EditorBlueprintResources/ActorMacros.Switch Has Authority`
    (:`Authority`
      (`self.ButtonAnimation` _v001_ordenador_posicionado_boton7_4_ (`KismetStringLibrary.Conv_StringToInt` (`KismetStringLibrary.Conv_NameToString` (`|GetArrayItem` (`ActorComponent.ComponentTags` OverlappedComponent))))))))

(event `self.Box_9.OnComponentEndOverlap`
  (params (OverlappedComponent :type "PrimitiveComponent Object Reference") (OtherActor :type "Actor Object Reference") (OtherComp :type "PrimitiveComponent Object Reference") (OtherBodyIndex :type Integer))
  (bind _v001_ordenador_posicionado_boton8_9_ (`self.v001_Ordenador_Posicionado_Boton8(9)`))
  (bind (_relativelocation_x _relativelocation_y _relativelocation_z) (`KismetMathLibrary.BreakVector` (`SceneComponent.RelativeLocation` _v001_ordenador_posicionado_boton8_9_)))
  ;[1 0.5511 0] Retorna a la posicion inical los botones cuando el objeto deja de estar encima
  (`KismetSystemLibrary.MoveComponentTo` _v001_ordenador_posicionado_boton8_9_ (`KismetMathLibrary.MakeVector` 0.0 0.0 (`KismetMathLibrary.FClamp` (+ _relativelocation_z 0.2) -0.4 0.0)) (struct) false false (`self.MovementSeconds`)))

(event `self.Box_9.OnComponentBeginOverlap`
  (params (OverlappedComponent :type "PrimitiveComponent Object Reference") (OtherActor :type "Actor Object Reference") (OtherComp :type "PrimitiveComponent Object Reference") (OtherBodyIndex :type Integer) (bFromSweep :type Boolean) (SweepResult :type "HitResult Structure (by ref)"))
  (bind _v001_ordenador_posicionado_boton8_9_ (`self.v001_Ordenador_Posicionado_Boton8(9)`))
  (bind (_relativelocation_x _relativelocation_y _relativelocation_z) (`KismetMathLibrary.BreakVector` (`SceneComponent.RelativeLocation` _v001_ordenador_posicionado_boton8_9_)))
  ;[1 0.5511 0] Cuando se pulse un botón lo mueve se llama al metodo ButtonAnimation pasandole el boton y el numero que tiene
  (`KismetSystemLibrary.MoveComponentTo` _v001_ordenador_posicionado_boton8_9_ (`KismetMathLibrary.MakeVector` 0.0 0.0 (`KismetMathLibrary.FClamp` (- _relativelocation_z 0.2) -0.4 0.0)) (struct) false false (`self.MovementSeconds`))
  (`self.ButtonAnimation` _v001_ordenador_posicionado_boton8_9_ (`KismetStringLibrary.Conv_StringToInt` (`KismetStringLibrary.Conv_NameToString` (`|GetArrayItem` (`ActorComponent.ComponentTags` OverlappedComponent))))))

(event `self.Box_8.OnComponentEndOverlap`
  (params (OverlappedComponent :type "PrimitiveComponent Object Reference") (OtherActor :type "Actor Object Reference") (OtherComp :type "PrimitiveComponent Object Reference") (OtherBodyIndex :type Integer))
  (bind _v001_ordenador_posicionado_boton9_8_ (`self.v001_Ordenador_Posicionado_Boton9(8)`))
  (bind (_relativelocation_x _relativelocation_y _relativelocation_z) (`KismetMathLibrary.BreakVector` (`SceneComponent.RelativeLocation` _v001_ordenador_posicionado_boton9_8_)))
  ;[1 0.5511 0] Retorna a la posicion inical los botones cuando el objeto deja de estar encima
  (`KismetSystemLibrary.MoveComponentTo` _v001_ordenador_posicionado_boton9_8_ (`KismetMathLibrary.MakeVector` 0.0 0.0 (`KismetMathLibrary.FClamp` (+ _relativelocation_z 0.2) -0.4 0.0)) (struct) false false (`self.MovementSeconds`)))

(event `self.Box_8.OnComponentBeginOverlap`
  (params (OverlappedComponent :type "PrimitiveComponent Object Reference") (OtherActor :type "Actor Object Reference") (OtherComp :type "PrimitiveComponent Object Reference") (OtherBodyIndex :type Integer) (bFromSweep :type Boolean) (SweepResult :type "HitResult Structure (by ref)"))
  (bind _v001_ordenador_posicionado_boton9_8_ (`self.v001_Ordenador_Posicionado_Boton9(8)`))
  (bind (_relativelocation_x _relativelocation_y _relativelocation_z) (`KismetMathLibrary.BreakVector` (`SceneComponent.RelativeLocation` _v001_ordenador_posicionado_boton9_8_)))
  ;[1 0.5511 0] Cuando se pulse un botón lo mueve se llama al metodo ButtonAnimation pasandole el boton y el numero que tiene
  (`KismetSystemLibrary.MoveComponentTo` _v001_ordenador_posicionado_boton9_8_ (`KismetMathLibrary.MakeVector` 0.0 0.0 (`KismetMathLibrary.FClamp` (- _relativelocation_z 0.2) -0.4 0.0)) (struct) false false (`self.MovementSeconds`))
  (`self.ButtonAnimation` _v001_ordenador_posicionado_boton9_8_ (`KismetStringLibrary.Conv_StringToInt` (`KismetStringLibrary.Conv_NameToString` (`|GetArrayItem` (`ActorComponent.ComponentTags` OverlappedComponent))))))

(event `self.Box_0.OnComponentEndOverlap`
  (params (OverlappedComponent :type "PrimitiveComponent Object Reference") (OtherActor :type "Actor Object Reference") (OtherComp :type "PrimitiveComponent Object Reference") (OtherBodyIndex :type Integer))
  (bind _v001_ordenador_posicionado_boton11_0_ (`self.v001_Ordenador_Posicionado_Boton11(0)`))
  (bind (_relativelocation_x _relativelocation_y _relativelocation_z) (`KismetMathLibrary.BreakVector` (`SceneComponent.RelativeLocation` _v001_ordenador_posicionado_boton11_0_)))
  ;[1 0.5511 0] Retorna a la posicion inical los botones cuando el objeto deja de estar encima
  (`KismetSystemLibrary.MoveComponentTo` _v001_ordenador_posicionado_boton11_0_ (`KismetMathLibrary.MakeVector` 0.0 0.0 (`KismetMathLibrary.FClamp` (+ _relativelocation_z 0.2) -0.4 0.0)) (struct) false false (`self.MovementSeconds`)))

(event `self.Box_3.OnComponentBeginOverlap`
  (params (OverlappedComponent :type "PrimitiveComponent Object Reference") (OtherActor :type "Actor Object Reference") (OtherComp :type "PrimitiveComponent Object Reference") (OtherBodyIndex :type Integer) (bFromSweep :type Boolean) (SweepResult :type "HitResult Structure (by ref)"))
  (bind _v001_ordenador_posicionado_boton2_3_ (`self.v001_Ordenador_Posicionado_Boton2(3)`))
  (bind (_relativelocation_x _relativelocation_y _relativelocation_z) (`KismetMathLibrary.BreakVector` (`SceneComponent.RelativeLocation` _v001_ordenador_posicionado_boton2_3_)))
  ;[1 0.5511 0] Cuando se pulse un botón lo mueve se llama al metodo ButtonAnimation pasandole el boton y el numero que tiene
  (`KismetSystemLibrary.MoveComponentTo` _v001_ordenador_posicionado_boton2_3_ (`KismetMathLibrary.MakeVector` 0.0 0.0 (`KismetMathLibrary.FClamp` (- _relativelocation_z 0.2) -0.4 0.0)) (struct) false false (`self.MovementSeconds`))
  (`self.ButtonAnimation` _v001_ordenador_posicionado_boton2_3_ (`KismetStringLibrary.Conv_StringToInt` (`KismetStringLibrary.Conv_NameToString` (`|GetArrayItem` (`ActorComponent.ComponentTags` OverlappedComponent))))))

(event `ButtonReturnPosition`
  (params (Button :type "StaticMeshComponent Object Reference") (Box :type "BoxComponent Object Reference") (BoxOverlap :type Boolean))
  ;[1 0.5511 0] Retorna a la posicion inical los botones cuando el objeto deja de estar encima
)

(event `self.Box_7.OnComponentEndOverlap`
  (params (OverlappedComponent :type "PrimitiveComponent Object Reference") (OtherActor :type "Actor Object Reference") (OtherComp :type "PrimitiveComponent Object Reference") (OtherBodyIndex :type Integer))
  (bind _v001_ordenador_posicionado_boton10_7_ (`self.v001_Ordenador_Posicionado_Boton10(7)`))
  (bind (_relativelocation_x _relativelocation_y _relativelocation_z) (`KismetMathLibrary.BreakVector` (`SceneComponent.RelativeLocation` _v001_ordenador_posicionado_boton10_7_)))
  ;[1 0.5511 0] Retorna a la posicion inical los botones cuando el objeto deja de estar encima
  (`KismetSystemLibrary.MoveComponentTo` _v001_ordenador_posicionado_boton10_7_ (`KismetMathLibrary.MakeVector` 0.0 0.0 (`KismetMathLibrary.FClamp` (+ _relativelocation_z 0.2) -0.4 0.0)) (struct) false false (`self.MovementSeconds`)))

(event `self.Box_2.OnComponentBeginOverlap`
  (params (OverlappedComponent :type "PrimitiveComponent Object Reference") (OtherActor :type "Actor Object Reference") (OtherComp :type "PrimitiveComponent Object Reference") (OtherBodyIndex :type Integer) (bFromSweep :type Boolean) (SweepResult :type "HitResult Structure (by ref)"))
  (bind _v001_ordenador_posicionado_boton3_2_ (`self.v001_Ordenador_Posicionado_Boton3(2)`))
  (bind (_relativelocation_x _relativelocation_y _relativelocation_z) (`KismetMathLibrary.BreakVector` (`SceneComponent.RelativeLocation` _v001_ordenador_posicionado_boton3_2_)))
  ;[1 0.5511 0] Cuando se pulse un botón lo mueve se llama al metodo ButtonAnimation pasandole el boton y el numero que tiene
  (`KismetSystemLibrary.MoveComponentTo` _v001_ordenador_posicionado_boton3_2_ (`KismetMathLibrary.MakeVector` 0.0 0.0 (`KismetMathLibrary.FClamp` (- _relativelocation_z 0.2) -0.4 0.0)) (struct) false false (`self.MovementSeconds`))
  (`self.ButtonAnimation` _v001_ordenador_posicionado_boton3_2_ (`KismetStringLibrary.Conv_StringToInt` (`KismetStringLibrary.Conv_NameToString` (`|GetArrayItem` (`ActorComponent.ComponentTags` OverlappedComponent))))))

(event `self.Box_ok.OnComponentEndOverlap`
  (params (OverlappedComponent :type "PrimitiveComponent Object Reference") (OtherActor :type "Actor Object Reference") (OtherComp :type "PrimitiveComponent Object Reference") (OtherBodyIndex :type Integer))
  (bind _v001_ordenador_posicionado_boton1_ok_ (`self.v001_Ordenador_Posicionado_Boton1(ok)`))
  (bind (_relativelocation_x _relativelocation_y _relativelocation_z) (`KismetMathLibrary.BreakVector` (`SceneComponent.RelativeLocation` _v001_ordenador_posicionado_boton1_ok_)))
  ;[1 0.5511 0] Retorna a la posicion inical los botones cuando el objeto deja de estar encima
  (`KismetSystemLibrary.MoveComponentTo` _v001_ordenador_posicionado_boton1_ok_ (`KismetMathLibrary.MakeVector` 0.0 0.0 (`KismetMathLibrary.FClamp` (+ _relativelocation_z 0.2) -0.4 0.0)) (struct) false false (`self.MovementSeconds`)))

(event `self.Box_7.OnComponentBeginOverlap`
  (params (OverlappedComponent :type "PrimitiveComponent Object Reference") (OtherActor :type "Actor Object Reference") (OtherComp :type "PrimitiveComponent Object Reference") (OtherBodyIndex :type Integer) (bFromSweep :type Boolean) (SweepResult :type "HitResult Structure (by ref)"))
  (bind _v001_ordenador_posicionado_boton10_7_ (`self.v001_Ordenador_Posicionado_Boton10(7)`))
  (bind (_relativelocation_x _relativelocation_y _relativelocation_z) (`KismetMathLibrary.BreakVector` (`SceneComponent.RelativeLocation` _v001_ordenador_posicionado_boton10_7_)))
  ;[1 0.5511 0] Cuando se pulse un botón lo mueve se llama al metodo ButtonAnimation pasandole el boton y el numero que tiene
  (`KismetSystemLibrary.MoveComponentTo` _v001_ordenador_posicionado_boton10_7_ (`KismetMathLibrary.MakeVector` 0.0 0.0 (`KismetMathLibrary.FClamp` (- _relativelocation_z 0.2) -0.4 0.0)))
  (`self.ButtonAnimation` _v001_ordenador_posicionado_boton10_7_ (`KismetStringLibrary.Conv_StringToInt` (`KismetStringLibrary.Conv_NameToString` (`|GetArrayItem` (`ActorComponent.ComponentTags` OverlappedComponent))))))

(event `self.Box_6.OnComponentEndOverlap`
  (params (OverlappedComponent :type "PrimitiveComponent Object Reference") (OtherActor :type "Actor Object Reference") (OtherComp :type "PrimitiveComponent Object Reference") (OtherBodyIndex :type Integer))
  (bind _v001_ordenador_posicionado_boton5_6_ (`self.v001_Ordenador_Posicionado_Boton5(6)`))
  (bind (_relativelocation_x _relativelocation_y _relativelocation_z) (`KismetMathLibrary.BreakVector` (`SceneComponent.RelativeLocation` _v001_ordenador_posicionado_boton5_6_)))
  ;[1 0.5511 0] Retorna a la posicion inical los botones cuando el objeto deja de estar encima
  (`KismetSystemLibrary.MoveComponentTo` _v001_ordenador_posicionado_boton5_6_ (`KismetMathLibrary.MakeVector` 0.0 0.0 (`KismetMathLibrary.FClamp` (+ _relativelocation_z 0.2) -0.4 0.0)) (struct) false false (`self.MovementSeconds`)))

(event `self.Box_delete.OnComponentEndOverlap`
  (params (OverlappedComponent :type "PrimitiveComponent Object Reference") (OtherActor :type "Actor Object Reference") (OtherComp :type "PrimitiveComponent Object Reference") (OtherBodyIndex :type Integer))
  (bind _v001_ordenador_posicionado_boton12_delete_ (`self.v001_Ordenador_Posicionado_Boton12(delete)`))
  (bind (_relativelocation_x _relativelocation_y _relativelocation_z) (`KismetMathLibrary.BreakVector` (`SceneComponent.RelativeLocation` _v001_ordenador_posicionado_boton12_delete_)))
  ;[1 0.5511 0] Retorna a la posicion inical los botones cuando el objeto deja de estar encima
  (`KismetSystemLibrary.MoveComponentTo` _v001_ordenador_posicionado_boton12_delete_ (`KismetMathLibrary.MakeVector` 0.0 0.0 (`KismetMathLibrary.FClamp` (+ _relativelocation_z 0.2) -0.4 0.0)) (struct) false false (`self.MovementSeconds`)))

(event `self.Box_1.OnComponentBeginOverlap`
  (params (OverlappedComponent :type "PrimitiveComponent Object Reference") (OtherActor :type "Actor Object Reference") (OtherComp :type "PrimitiveComponent Object Reference") (OtherBodyIndex :type Integer) (bFromSweep :type Boolean) (SweepResult :type "HitResult Structure (by ref)"))
  (bind _v001_ordenador_posicionado_boton4_1_ (`self.v001_Ordenador_Posicionado_Boton4(1)`))
  (bind (_relativelocation_x _relativelocation_y _relativelocation_z) (`KismetMathLibrary.BreakVector` (`SceneComponent.RelativeLocation` _v001_ordenador_posicionado_boton4_1_)))
  ;[1 0.5511 0] Cuando se pulse un botón lo mueve se llama al metodo ButtonAnimation pasandole el boton y el numero que tiene
  (`KismetSystemLibrary.MoveComponentTo` _v001_ordenador_posicionado_boton4_1_ (`KismetMathLibrary.MakeVector` 0.0 0.0 (`KismetMathLibrary.FClamp` (- _relativelocation_z 0.2) -0.4 0.0)) (struct) false false (`self.MovementSeconds`))
  (`self.ButtonAnimation` _v001_ordenador_posicionado_boton4_1_ (`KismetStringLibrary.Conv_StringToInt` (`KismetStringLibrary.Conv_NameToString` (`|GetArrayItem` (`ActorComponent.ComponentTags` OverlappedComponent))))))

(event `self.Box_6.OnComponentBeginOverlap`
  (params (OverlappedComponent :type "PrimitiveComponent Object Reference") (OtherActor :type "Actor Object Reference") (OtherComp :type "PrimitiveComponent Object Reference") (OtherBodyIndex :type Integer) (bFromSweep :type Boolean) (SweepResult :type "HitResult Structure (by ref)"))
  (bind _v001_ordenador_posicionado_boton5_6_ (`self.v001_Ordenador_Posicionado_Boton5(6)`))
  (bind (_relativelocation_x _relativelocation_y _relativelocation_z) (`KismetMathLibrary.BreakVector` (`SceneComponent.RelativeLocation` _v001_ordenador_posicionado_boton5_6_)))
  ;[1 0.5511 0] Cuando se pulse un botón lo mueve se llama al metodo ButtonAnimation pasandole el boton y el numero que tiene
  (`KismetSystemLibrary.MoveComponentTo` _v001_ordenador_posicionado_boton5_6_ (`KismetMathLibrary.MakeVector` 0.0 0.0 (`KismetMathLibrary.FClamp` (- _relativelocation_z 0.2) -0.4 0.0)) (struct) false false (`self.MovementSeconds`))
  (`self.ButtonAnimation` _v001_ordenador_posicionado_boton5_6_ (`KismetStringLibrary.Conv_StringToInt` (`KismetStringLibrary.Conv_NameToString` (`|GetArrayItem` (`ActorComponent.ComponentTags` OverlappedComponent))))))

(event `self.Box_5.OnComponentEndOverlap`
  (params (OverlappedComponent :type "PrimitiveComponent Object Reference") (OtherActor :type "Actor Object Reference") (OtherComp :type "PrimitiveComponent Object Reference") (OtherBodyIndex :type Integer))
  (bind _v001_ordenador_posicionado_boton6_5_ (`self.v001_Ordenador_Posicionado_Boton6(5)`))
  (bind (_relativelocation_x _relativelocation_y _relativelocation_z) (`KismetMathLibrary.BreakVector` (`SceneComponent.RelativeLocation` _v001_ordenador_posicionado_boton6_5_)))
  ;[1 0.5511 0] Retorna a la posicion inical los botones cuando el objeto deja de estar encima
  (`KismetSystemLibrary.MoveComponentTo` _v001_ordenador_posicionado_boton6_5_ (`KismetMathLibrary.MakeVector` 0.0 0.0 (`KismetMathLibrary.FClamp` (+ _relativelocation_z 0.2) -0.4 0.0))))

(event `self.Box_3.OnComponentEndOverlap`
  (params (OverlappedComponent :type "PrimitiveComponent Object Reference") (OtherActor :type "Actor Object Reference") (OtherComp :type "PrimitiveComponent Object Reference") (OtherBodyIndex :type Integer))
  (bind _v001_ordenador_posicionado_boton2_3_ (`self.v001_Ordenador_Posicionado_Boton2(3)`))
  (bind (_relativelocation_x _relativelocation_y _relativelocation_z) (`KismetMathLibrary.BreakVector` (`SceneComponent.RelativeLocation` _v001_ordenador_posicionado_boton2_3_)))
  ;[1 0.5511 0] Retorna a la posicion inical los botones cuando el objeto deja de estar encima
  (`KismetSystemLibrary.MoveComponentTo` _v001_ordenador_posicionado_boton2_3_ (`KismetMathLibrary.MakeVector` 0.0 0.0 (`KismetMathLibrary.FClamp` (+ _relativelocation_z 0.2) -0.4 0.0)) (struct) false false (`self.MovementSeconds`)))

(event `self.Box_0.OnComponentBeginOverlap`
  (params (OverlappedComponent :type "PrimitiveComponent Object Reference") (OtherActor :type "Actor Object Reference") (OtherComp :type "PrimitiveComponent Object Reference") (OtherBodyIndex :type Integer) (bFromSweep :type Boolean) (SweepResult :type "HitResult Structure (by ref)"))
  (bind _v001_ordenador_posicionado_boton11_0_ (`self.v001_Ordenador_Posicionado_Boton11(0)`))
  (bind (_relativelocation_x _relativelocation_y _relativelocation_z) (`KismetMathLibrary.BreakVector` (`SceneComponent.RelativeLocation` _v001_ordenador_posicionado_boton11_0_)))
  ;[1 0.5511 0] Cuando se pulse un botón lo mueve se llama al metodo ButtonAnimation pasandole el boton y el numero que tiene
  (`KismetSystemLibrary.MoveComponentTo` _v001_ordenador_posicionado_boton11_0_ (`KismetMathLibrary.MakeVector` 0.0 0.0 (`KismetMathLibrary.FClamp` (- _relativelocation_z 0.2) -0.4 0.0)) (struct) false false (`self.MovementSeconds`))
  (`self.ButtonAnimation` _v001_ordenador_posicionado_boton11_0_ (`KismetStringLibrary.Conv_StringToInt` (`KismetStringLibrary.Conv_NameToString` (`|GetArrayItem` (`ActorComponent.ComponentTags` OverlappedComponent))))))

(event `self.Box_5.OnComponentBeginOverlap`
  (params (OverlappedComponent :type "PrimitiveComponent Object Reference") (OtherActor :type "Actor Object Reference") (OtherComp :type "PrimitiveComponent Object Reference") (OtherBodyIndex :type Integer) (bFromSweep :type Boolean) (SweepResult :type "HitResult Structure (by ref)"))
  (bind _v001_ordenador_posicionado_boton6_5_ (`self.v001_Ordenador_Posicionado_Boton6(5)`))
  (bind (_relativelocation_x _relativelocation_y _relativelocation_z) (`KismetMathLibrary.BreakVector` (`SceneComponent.RelativeLocation` _v001_ordenador_posicionado_boton6_5_)))
  ;[1 0.5511 0] Cuando se pulse un botón lo mueve se llama al metodo ButtonAnimation pasandole el boton y el numero que tiene
  (`KismetSystemLibrary.MoveComponentTo` _v001_ordenador_posicionado_boton6_5_ (`KismetMathLibrary.MakeVector` 0.0 0.0 (`KismetMathLibrary.FClamp` (- _relativelocation_z 0.2) -0.4 0.0)) (struct) false false (`self.MovementSeconds`))
  (`self.ButtonAnimation` _v001_ordenador_posicionado_boton6_5_ (`KismetStringLibrary.Conv_StringToInt` (`KismetStringLibrary.Conv_NameToString` (`|GetArrayItem` (`ActorComponent.ComponentTags` OverlappedComponent))))))

(event `self.Box_4.OnComponentEndOverlap`
  (params (OverlappedComponent :type "PrimitiveComponent Object Reference") (OtherActor :type "Actor Object Reference") (OtherComp :type "PrimitiveComponent Object Reference") (OtherBodyIndex :type Integer))
  (bind _v001_ordenador_posicionado_boton7_4_ (`self.v001_Ordenador_Posicionado_Boton7(4)`))
  (bind (_relativelocation_x _relativelocation_y _relativelocation_z) (`KismetMathLibrary.BreakVector` (`SceneComponent.RelativeLocation` _v001_ordenador_posicionado_boton7_4_)))
  ;[1 0.5511 0] Retorna a la posicion inical los botones cuando el objeto deja de estar encima
  (`KismetSystemLibrary.MoveComponentTo` _v001_ordenador_posicionado_boton7_4_ (`KismetMathLibrary.MakeVector` 0.0 0.0 (`KismetMathLibrary.FClamp` (+ _relativelocation_z 0.2) -0.4 0.0))))

(event `self.Box_2.OnComponentEndOverlap`
  (params (OverlappedComponent :type "PrimitiveComponent Object Reference") (OtherActor :type "Actor Object Reference") (OtherComp :type "PrimitiveComponent Object Reference") (OtherBodyIndex :type Integer))
  (bind _v001_ordenador_posicionado_boton3_2_ (`self.v001_Ordenador_Posicionado_Boton3(2)`))
  (bind (_relativelocation_x _relativelocation_y _relativelocation_z) (`KismetMathLibrary.BreakVector` (`SceneComponent.RelativeLocation` _v001_ordenador_posicionado_boton3_2_)))
  ;[1 0.5511 0] Retorna a la posicion inical los botones cuando el objeto deja de estar encima
  (`KismetSystemLibrary.MoveComponentTo` _v001_ordenador_posicionado_boton3_2_ (`KismetMathLibrary.MakeVector` 0.0 0.0 (`KismetMathLibrary.FClamp` (+ _relativelocation_z 0.2) -0.4 0.0)) (struct) false false (`self.MovementSeconds`)))

(event `self.Box_ok.OnComponentBeginOverlap`
  (params (OverlappedComponent :type "PrimitiveComponent Object Reference") (OtherActor :type "Actor Object Reference") (OtherComp :type "PrimitiveComponent Object Reference") (OtherBodyIndex :type Integer) (bFromSweep :type Boolean) (SweepResult :type "HitResult Structure (by ref)"))
  (bind (_relativelocation_x _relativelocation_y _relativelocation_z) (`KismetMathLibrary.BreakVector` (`SceneComponent.RelativeLocation` (`self.v001_Ordenador_Posicionado_Boton1(ok)`))))
  ;[1 0.5342 0] Cuando se pulsa el boton ok(la colision) mueve el boton hacia atras y llama al evento CheckCorrectCode del WID_PantallaCajaFuerte
  (`KismetSystemLibrary.MoveComponentTo` (`self.v001_Ordenador_Posicionado_Boton1(ok)`) (`KismetMathLibrary.MakeVector` 0.0 0.0 (`KismetMathLibrary.FClamp` (- _relativelocation_z 0.2) -0.4 0.0)) (struct) false false (`self.MovementSeconds`))
  (cast `/Game/Widgets/WID_PantallaOrdenador` (`WidgetComponent.GetWidget` (`self.Widget`)))
  (if (not (`self.Open?`))
    (`self.CheckCorrectCode`)))

(event `ButtonAnimation`
  (params (BotonPresionado :type "StaticMeshComponent Object Reference") (Numero :type Integer))
  (bind _contador (`self.Contador`))
  ;[1 0.2217 0.09193] Mueve el boton correspondiente y llama al metodo ChangeValue del WID_PantallaCajaFuerte
  (cast `/Game/Widgets/WID_PantallaOrdenador` (`WidgetComponent.GetWidget` (`self.Widget`)))
  (`self.ChangeValue` Numero _contador)
  (if (not (== _contador 4))
    (`/Engine/EditorBlueprintResources/StandardMacros.IncrementInt` _contador)))

(event `self.Box_delete.OnComponentBeginOverlap`
  (params (OverlappedComponent :type "PrimitiveComponent Object Reference") (OtherActor :type "Actor Object Reference") (OtherComp :type "PrimitiveComponent Object Reference") (OtherBodyIndex :type Integer) (bFromSweep :type Boolean) (SweepResult :type "HitResult Structure (by ref)"))
  (bind _contador (`self.Contador`))
  (bind (_relativelocation_x _relativelocation_y _relativelocation_z) (`KismetMathLibrary.BreakVector` (`SceneComponent.RelativeLocation` (`self.v001_Ordenador_Posicionado_Boton12(delete)`))))
  ;[1 0.5342 0] Cuando se pulsa el boton delete(la colision) mueve el boton hacia atras y llama al evento Reset del WID_PantallaCajaFuerte
  (`KismetSystemLibrary.MoveComponentTo` (`self.v001_Ordenador_Posicionado_Boton12(delete)`) (`KismetMathLibrary.MakeVector` 0.0 0.0 (`KismetMathLibrary.FClamp` (- _relativelocation_z 0.2) -0.4 0.0)) (struct) false false (`self.MovementSeconds`))
  (if (not (== _contador 0))
    (bind _result (`/Engine/EditorBlueprintResources/StandardMacros.DecrementInt` _contador)
      (:`  `
        (`self.Reset` _result)))))

(event `SetOpen`
  ;[1 0.1885 0.219] Pone la variable Open? en true y añade un sonido al boton
  (set `self.Open?` true)
  (`GameplayStatics.PlaySound2D` "/Engine/EngineSounds/1kSineTonePing.1kSineTonePing" 1.0 1.0 0.0 null null))

(event `OpenDoor`
  ;[1 0.212 0.202] Abre la puerta, cambia el material de la pantalla por uno verde y  hace sonar un sonido
)

(event `ResetColor`
  ;[1 0.1885 0.219] Resetea el color del marco y setea el contador a 0
)

(event `PostitContraseña`
  (params (Players :type Integer))
  (bind _aswid_post_it (cast `/Game/Widgets/WID_PostIt` (`WidgetComponent.GetWidget` (`self.PostIt`))))
  (`/Game/Widgets/WID_PostIt.ChangeValue` _aswid_post_it Players))

(event `SetErrorColor`
  ;[1 0.2135 0.2392] Pone color rojo cuando se introduce un codigo incorrecto
)

(event `SetCode`
  ;[1 1 1] Guarda el codigo actual en una variable
  (bind _aswid_pantalla_ordenador (cast `/Game/Widgets/WID_PantallaOrdenador` (`WidgetComponent.GetWidget` (`self.Widget`))))
  (set `/Game/Widgets/WID_PantallaOrdenador.CodigoIntroducido` (`KismetStringLibrary.Concat_StrStr` (`KismetTextLibrary.Conv_TextToString` (`TextBlock.Text` (`/Game/Widgets/WID_PantallaOrdenador.PWD_1` _aswid_pantalla_ordenador))) (`KismetTextLibrary.Conv_TextToString` (`TextBlock.Text` (`/Game/Widgets/WID_PantallaOrdenador.PWD_2` _aswid_pantalla_ordenador))) (`KismetTextLibrary.Conv_TextToString` (`TextBlock.Text` (`/Game/Widgets/WID_PantallaOrdenador.PWD_3` _aswid_pantalla_ordenador))) (`KismetTextLibrary.Conv_TextToString` (`TextBlock.Text` (`/Game/Widgets/WID_PantallaOrdenador.PWD_4` _aswid_pantalla_ordenador)))) _aswid_pantalla_ordenador))

(event `ChangeValue`
  (params (Num :type Integer) (Position :type Integer))
  ;[1 1 1] Muestra el numero introducido en el txt correspondiente
  (`self.ChangeValueMulticast` Num Position))

(event `ChangeValueMulticast`
  (params (Num :type Integer) (Position :type Integer))
  ;[1 1 1] Muestra el numero introducido en el txt correspondiente
  (bind _aswid_pantalla_ordenador (cast `/Game/Widgets/WID_PantallaOrdenador` (`WidgetComponent.GetWidget` (`self.Widget`))))
  (switch `int` Position
    (:`0`
      (`TextBlock.SetText` (`/Game/Widgets/WID_PantallaOrdenador.PWD_1` _aswid_pantalla_ordenador) (`KismetTextLibrary.Conv_IntToText` Num)))
    (:`1`
      (`TextBlock.SetText` (`/Game/Widgets/WID_PantallaOrdenador.PWD_2` _aswid_pantalla_ordenador) (`KismetTextLibrary.Conv_IntToText` Num)))
    (:`2`
      (`TextBlock.SetText` (`/Game/Widgets/WID_PantallaOrdenador.PWD_3` _aswid_pantalla_ordenador) (`KismetTextLibrary.Conv_IntToText` Num)))
    (:`3`
      (`TextBlock.SetText` (`/Game/Widgets/WID_PantallaOrdenador.PWD_4` _aswid_pantalla_ordenador) (`KismetTextLibrary.Conv_IntToText` Num))))
  (`self.SetCode`))

(event `CheckCorrectCode`
  ;[1 1 1] Comprueba si el código introducido es correcto
  (`self.CheckCorrectCodeMulticast`)
  (bind _aswid_pantalla_ordenador (cast `/Game/Widgets/WID_PantallaOrdenador` (`WidgetComponent.GetWidget` (`self.Widget`)) :!label _label))
  (if (`KismetStringLibrary.EqualEqual_StrStr` (`/Game/Widgets/WID_PantallaOrdenador.CodigoIntroducido` _aswid_pantalla_ordenador) (`self.CodigoCorrecto`))
    (bind _returnvalue (`GameplayStatics.GetActorOfClass` "/Game/Blueprints/BP_Mesilla_ordenador.BP_Mesilla_ordenador_C"))
    (`/Game/Blueprints/BP_Mesilla_ordenador.AbrirCajon` _returnvalue)
    (bind _pwd_1 (`/Game/Widgets/WID_PantallaOrdenador.PWD_1` _aswid_pantalla_ordenador))
    (`TextBlock.SetColorAndOpacity` _pwd_1 (make `SlateColor` (struct :`R` 0.192751 :`G` 1.0 :`A` 1.0)))
    (`TextBlock.SetColorAndOpacity` (`/Game/Widgets/WID_PantallaOrdenador.PWD_2` _aswid_pantalla_ordenador) (make `SlateColor` (struct :`R` 0.192751 :`G` 1.0 :`A` 1.0)))
    (`TextBlock.SetColorAndOpacity` (`/Game/Widgets/WID_PantallaOrdenador.PWD_3` _aswid_pantalla_ordenador) (make `SlateColor` (struct :`R` 0.192751 :`G` 1.0 :`A` 1.0)))
    (`TextBlock.SetColorAndOpacity` (`/Game/Widgets/WID_PantallaOrdenador.PWD_4` _aswid_pantalla_ordenador) (make `SlateColor` (struct :`R` 0.192751 :`G` 1.0 :`A` 1.0)))
    (`TextBlock.SetText` _pwd_1 "O")
    (bind _pwd_2 (`/Game/Widgets/WID_PantallaOrdenador.PWD_2` _aswid_pantalla_ordenador))
    (`TextBlock.SetText` _pwd_2 "P")
    (bind _pwd_3 (`/Game/Widgets/WID_PantallaOrdenador.PWD_3` _aswid_pantalla_ordenador))
    (`TextBlock.SetText` _pwd_3 "E")
    (bind _pwd_4 (`/Game/Widgets/WID_PantallaOrdenador.PWD_4` _aswid_pantalla_ordenador))
    (`TextBlock.SetText` _pwd_4 "N")
    (else
      (`TextBlock.SetColorAndOpacity` _pwd_1 (make `SlateColor` (struct :`R` 1.0 :`B` 0.026767 :`A` 1.0)))
      (`TextBlock.SetColorAndOpacity` _pwd_2 (make `SlateColor` (struct :`R` 1.0 :`B` 0.026767 :`A` 1.0)))
      (`TextBlock.SetColorAndOpacity` _pwd_3 (make `SlateColor` (struct :`R` 1.0 :`B` 0.026767 :`A` 1.0)))
      (`TextBlock.SetColorAndOpacity` _pwd_4 (make `SlateColor` (struct :`R` 1.0 :`B` 0.026767 :`A` 1.0)))
      (`KismetSystemLibrary.Delay` 2.0)
      (`TextBlock.SetColorAndOpacity` _pwd_1 (make `SlateColor` (struct :`R` 0.070588 :`B` 1.0 :`A` 1.0)))
      (`TextBlock.SetColorAndOpacity` _pwd_2 (make `SlateColor` (struct :`R` 1.0 :`G` 0.098039 :`B` 0.039216 :`A` 1.0)))
      (`TextBlock.SetColorAndOpacity` _pwd_3 (make `SlateColor` (struct :`R` 0.176471 :`G` 1.0 :`A` 1.0)))
      (`TextBlock.SetColorAndOpacity` _pwd_4 (make `SlateColor` (struct :`R` 1.0 :`G` 0.019608 :`B` 0.788235 :`A` 1.0))))))

(event `CheckCorrectCodeMulticast`
  ;[1 1 1] Comprueba si el código introducido es correcto
  (goto _label))

(event `Reset`
  (params (cont :type Integer))
  ;[1 1 1] Resetea los numeros del codigo a 0
  (`self.ResetMulticast` cont))

(event `ResetMulticast`
  (params (cont :type Integer))
  ;[1 1 1] Resetea los numeros del codigo a 0
  (bind _aswid_pantalla_ordenador (cast `/Game/Widgets/WID_PantallaOrdenador` (`WidgetComponent.GetWidget` (`self.Widget`))))
  (switch `int` cont
    (:`0`
      (`TextBlock.SetText` (`/Game/Widgets/WID_PantallaOrdenador.PWD_1` _aswid_pantalla_ordenador) "_"))
    (:`1`
      (`TextBlock.SetText` (`/Game/Widgets/WID_PantallaOrdenador.PWD_2` _aswid_pantalla_ordenador) "_"))
    (:`2`
      (`TextBlock.SetText` (`/Game/Widgets/WID_PantallaOrdenador.PWD_3` _aswid_pantalla_ordenador) "_"))
    (:`3`
      (`TextBlock.SetText` (`/Game/Widgets/WID_PantallaOrdenador.PWD_4` _aswid_pantalla_ordenador) "_"))))

(event `self.ReceiveBeginPlay`)

(fn `UserConstructionScript`)