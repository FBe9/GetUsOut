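; BP_Cuadro is a VR-grabbable actor, apparently a picture frame, meant to move with the motion controller within limits.
; Grabbing stores the controller and starts a looping timer targeting "UpdateLocation", which is absent here; dropping clears both.
; UpdateMovement adds the controller's relative yaw to the Capsule's yaw, clamped between the local Y values of two Spline points.
; A variant setting Capsule Y location is disconnected.
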(event `self.GrabComponent.OnGrabbed`
  (params (`Motion Controller` :type "MotionControllerComponent Object Reference"))
  (set `self.Motion Controller` `Motion Controller`)
  (bind _returnvalue (`KismetSystemLibrary.K2_SetTimer` null "UpdateLocation" 0.01 true))
  (set `self.Timer` _returnvalue))

(event `self.GrabComponent.OnDropped`
  (`KismetSystemLibrary.K2_ClearAndInvalidateTimerHandle` (`self.Timer`))
  (set `self.Motion Controller` null))

(fn `UpdateMovement`
  (bind _capsule (`self.Capsule`))
  (bind _spline (`self.Spline`))
  (bind (_returnvalue_x _returnvalue_y) (`KismetMathLibrary.BreakVector` (`SplineComponent.GetLocationAtSplinePoint` _spline 1 "Local")))
  (bind (_returnvalue_x_2 _returnvalue_y_2) (`KismetMathLibrary.BreakVector` (`SplineComponent.GetLocationAtSplinePoint` _spline 0 "Local")))
  (bind (_relativerotation_roll _relativerotation_pitch _relativerotation_yaw) (`KismetMathLibrary.BreakRotator` (`SceneComponent.RelativeRotation` _capsule)))
  (`SceneComponent.K2_SetRelativeRotation` (`self.Capsule`) (`KismetMathLibrary.MakeRotator` _relativerotation_roll _relativerotation_pitch (`KismetMathLibrary.FClamp` (+ _relativerotation_yaw (.yaw (.rotation (`KismetMathLibrary.MakeRelativeTransform` (`SceneComponent.K2_GetComponentToWorld` (`self.Motion Controller`)) (`SceneComponent.K2_GetComponentToWorld` _capsule))))) _returnvalue_y_2 _returnvalue_y)) false false))

(fn `UserConstructionScript`)