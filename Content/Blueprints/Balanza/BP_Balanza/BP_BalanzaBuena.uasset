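; Balance scale puzzle that opens a drawer and the basement door when valid BP_Pesa weights balance both sides.
; Left and right box overlaps track total mass, and the clamped mass difference sets the animated pitch of beam and ropes.
; An empty scale tilts randomly, while a single loaded side tips to maximum, with its real mass cached.
; After the beam moves, a near-level pitch with valid objects solves the puzzle.
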(event `self.BoxRight.OnComponentBeginOverlap`
  (params (OverlappedComponent :type "PrimitiveComponent Object Reference") (OtherActor :type "Actor Object Reference") (OtherComp :type "PrimitiveComponent Object Reference") (OtherBodyIndex :type Integer) (bFromSweep :type Boolean) (SweepResult :type "HitResult Structure (by ref)"))
  (bind _massleftaux (`self.MassLeftAux`))
  ;[0.3467 1 0.6445] Setea las masas de los objetos que se han colocado en la balanza y llama al evento MoverBalanza
  (cast `/Game/Blueprints/Pesa/BP_Pesa/BP_Pesa` OtherActor
    (:`then`
      (set `self.ObjetoRightValido?` true))
    (:`CastFailed`
      (set `self.ObjetoRightValido?` false)))
  (bind _output_get (set `self.RealMassRight` (+ (`self.RealMassRight`) (`PrimitiveComponent.GetMass` OtherComp))))
  (set `self.ObjectRight?` true)
  (if (and (!= _massleftaux 0.0) (== (`self.MassRight`) 0.0))
    (set `self.MassLeft` _massleftaux)
    (set `self.MassLeftAux` 0.0))
  (set `self.MassRight` _output_get)
  (set `self.ObjetosValido?` (and (`self.ObjetoRightValido?`) (`self.ObjetoLeftValido?`)) :!label _label)
  (`self.MoveBalanza`))

(event `MoveBalanza`
  (bind _v005_balanza_ropes (`self.v005_Balanza_Ropes`))
  (bind _v005_balanza_ropes1 (`self.v005_Balanza_Ropes1`))
  (bind _v005_balanza_balanza_palo (`self.v005_Balanza_Balanza_Palo`))
  (bind (_relativerotation_roll _relativerotation_pitch _relativerotation_yaw) (`KismetMathLibrary.BreakRotator` (`SceneComponent.RelativeRotation` _v005_balanza_ropes)))
  (bind (_relativerotation_roll_2 _relativerotation_pitch_2 _relativerotation_yaw_2) (`KismetMathLibrary.BreakRotator` (`SceneComponent.RelativeRotation` _v005_balanza_balanza_palo)))
  (bind (_relativerotation_roll_3 _relativerotation_pitch_3 _relativerotation_yaw_3) (`KismetMathLibrary.BreakRotator` (`SceneComponent.RelativeRotation` _v005_balanza_ropes1)))
  ;[1 0.4282 0.1419] Llama a la funcion CheckRightLeft0 y la funcion CheckGrades y luego mueve la balanza en base al peso de los objetos y llama a la funcion CheckPuzleResuelto
  (`self.CheckIsObject`)
  (`self.CheckRightLeft0`)
  (set `self.Grados` (- (`self.MassLeft`) (`self.MassRight`)))
  (`self.CheckGrades`)
  (`GameplayStatics.PlaySoundAtLocation` null (`self.K2_GetActorLocation`) (struct) 1.0 1.0 0.0 null null null null)
  (`|ExecutionSequence`
    (:`then_0`
      (`KismetSystemLibrary.MoveComponentTo` _v005_balanza_ropes (`SceneComponent.RelativeLocation` _v005_balanza_ropes) (`KismetMathLibrary.MakeRotator` _relativerotation_roll (`self.Grados`) _relativerotation_yaw) false false 2.0))
    (:`then_1`
      (`KismetSystemLibrary.MoveComponentTo` _v005_balanza_balanza_palo (`SceneComponent.RelativeLocation` _v005_balanza_balanza_palo) (`KismetMathLibrary.MakeRotator` _relativerotation_roll_2 (`self.Grados`) _relativerotation_yaw_2) false false 2.0)
      (if (`self.CajonAbierto?`)
        _
        (elif (`self.ObjetosValido?`)
          (`self.CheckPuzleResuelto`))))
    (:`then_2`
      (`KismetSystemLibrary.MoveComponentTo` _v005_balanza_ropes1 (`SceneComponent.RelativeLocation` _v005_balanza_ropes1) (`KismetMathLibrary.MakeRotator` _relativerotation_roll_3 (`self.Grados`) _relativerotation_yaw_3) false false 2.0))))

(event `self.BoxLeft.OnComponentBeginOverlap`
  (params (OverlappedComponent :type "PrimitiveComponent Object Reference") (OtherActor :type "Actor Object Reference") (OtherComp :type "PrimitiveComponent Object Reference") (OtherBodyIndex :type Integer) (bFromSweep :type Boolean) (SweepResult :type "HitResult Structure (by ref)"))
  (bind _massrightaux (`self.MassRightAux`))
  ;[0.3467 1 0.6445] Setea las masas de los objetos que se han colocado en la balanza y llama al evento MoverBalanza
  (cast `/Game/Blueprints/Pesa/BP_Pesa/BP_Pesa` OtherActor
    (:`then`
      (set `self.ObjetoLeftValido?` true))
    (:`CastFailed`
      (set `self.ObjetoLeftValido?` false)))
  (bind _output_get (set `self.RealMassLeft` (+ (`self.RealMassLeft`) (`PrimitiveComponent.GetMass` OtherComp))))
  (set `self.ObjectLeft` true)
  (if (and (!= _massrightaux 0.0) (== (`self.MassLeft`) 0.0))
    (set `self.MassRight` _massrightaux)
    (set `self.MassRightAux` 0.0))
  (set `self.MassLeft` _output_get)
  (goto _label))

(event `self.BoxRight.OnComponentEndOverlap`
  (params (OverlappedComponent :type "PrimitiveComponent Object Reference") (OtherActor :type "Actor Object Reference") (OtherComp :type "PrimitiveComponent Object Reference") (OtherBodyIndex :type Integer))
  ;[0.3467 1 0.6445] Setea a 0 las masas de los objetos correspondientes cuando estos se quiten de la balanza y llama al evento MoverBalanza
  (cast `/Game/Blueprints/Pesa/BP_Pesa/BP_Pesa` OtherActor
    (:`then`
      _)
    (:`CastFailed`
      (set `self.ObjetoRightValido?` true)))
  (bind _output_get (set `self.RealMassRight` (- (`self.RealMassRight`) (`PrimitiveComponent.GetMass` OtherComp))))
  (if (not (> _output_get 0.0))
    (set `self.ObjectRight?` false))
  (set `self.MassRight` _output_get)
  (`self.MoveBalanza` :!label _label_2))

(event `self.BoxLeft.OnComponentEndOverlap`
  (params (OverlappedComponent :type "PrimitiveComponent Object Reference") (OtherActor :type "Actor Object Reference") (OtherComp :type "PrimitiveComponent Object Reference") (OtherBodyIndex :type Integer))
  ;[0.3467 1 0.6445] Setea a 0 las masas de los objetos correspondientes cuando estos se quiten de la balanza y llama al evento MoverBalanza
  (cast `/Game/Blueprints/Pesa/BP_Pesa/BP_Pesa` OtherActor
    (:`then`
      _)
    (:`CastFailed`
      (set `self.ObjetoLeftValido?` true)))
  (bind _output_get (set `self.RealMassLeft` (- (`self.RealMassLeft`) (`PrimitiveComponent.GetMass` OtherComp))))
  (if (not (> _output_get 0.0))
    (set `self.ObjectLeft` false))
  (set `self.MassLeft` _output_get)
  (goto _label_2))

(event `CheckPuzleResuelto`
  (bind (_relativerotation_roll _relativerotation_pitch) (`KismetMathLibrary.BreakRotator` (`SceneComponent.RelativeRotation` (`self.v005_Balanza_Balanza_Palo`))))
  ;[1 0.1779 0.1746] Comprueba si el puzzle se ha resuelto
  (if (and (!= (`self.MassRight`) 0.0) (!= (`self.MassLeft`) 0.0) (and (<= _relativerotation_pitch 0.01) (>= _relativerotation_pitch -0.01)))
    (bind _returnvalue (`GameplayStatics.GetActorOfClass` "/Game/Blueprints/Mesilla/MesillaBalanza/BP_Mesilla_Cubo_Balanza.BP_Mesilla_Cubo_Balanza_C"))
    (`/Game/Blueprints/Mesilla/MesillaBalanza/BP_Mesilla_Cubo_Balanza.AbrirCajon` _returnvalue)
    (bind _returnvalue_2 (`GameplayStatics.GetActorOfClass` "/Game/SotanoFInal/BP_PuertaSotano.BP_PuertaSotano_C"))
    (`/Game/SotanoFInal/BP_PuertaSotano.AbrirPuerta` _returnvalue_2)
    (set `self.CajonAbierto?` true)))

(event `CheckGrades`
  (bind _maxgrades (`self.MaxGrades`))
  (bind _grados (`self.Grados`))
  (bind _returnvalue (* _maxgrades -1.0))
  ;[1 0.1774 0.176] Comprueba que si los grados no pasen de los maximos permitidos (30 o -30)
  (if (> _grados _maxgrades)
    (set `self.Grados` _maxgrades)
    (elif (< _grados _returnvalue)
      (set `self.Grados` _returnvalue))))

(event `self.ReceiveBeginPlay`
  (bind _returnvalue (`KismetMathLibrary.RandomFloatInRange` 0.0 7.0))
  ;[0.3467 1 0.6445] Deja la balanza probablemente desbalanceada
  (set `self.MassLeft` _returnvalue)
  (set `self.MassRight` _returnvalue))

(event `CheckRightLeft0`
  (bind _returnvalue (`KismetMathLibrary.RandomFloatInRange` 0.0 7.0))
  (bind _maxgrades (`self.MaxGrades`))
  (bind _returnvalue_2 (== (`self.MassLeft`) 0.0))
  (bind _returnvalue_3 (== (`self.MassRight`) 0.0))
  ;[1 0.1774 0.176] Comprueba si las masas son iguales a 0 o si una de ellas es igual a 0. Si lo son se cambiaran los valores para que la balanza sea realista
  (if (and _returnvalue_2 _returnvalue_3)
    (set `self.MassLeft` _returnvalue)
    (set `self.MassRight` _returnvalue)
    (elif _returnvalue_2
      (set `self.MassRightAux` (`self.MassRight`))
      (set `self.MassRight` _maxgrades)
      (elif _returnvalue_3
        (set `self.MassLeftAux` (`self.MassLeft`))
        (set `self.MassLeft` _maxgrades)))))

(event `CheckIsObject`
  ;[1 0.1779 0.1746] Comprueba que si no hay objeto en la balanza este pase a ser 0
  (`|ExecutionSequence`
    (:`then_0`
      (if (not (`self.ObjectRight?`))
        (set `self.MassRight` 0.0)))
    (:`then_1`
      (if (not (`self.ObjectLeft`))
        (set `self.MassLeft` 0.0)))))

(fn `UserConstructionScript`)