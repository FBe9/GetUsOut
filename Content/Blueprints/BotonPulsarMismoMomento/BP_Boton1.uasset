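; BP_Boton1 is a pressure button, paired with BP_Boton2 to detect both being pressed at the same moment.
; An actor overlap prints a placeholder "Hello" if the first BP_Boton2 found has BotonClicked set, then sets its own flag.
; One timeline lerps the mesh slightly down from its BeginPlay location.
; A second timeline, played in reverse, raises it and clears the flag, so a press lasts only for the animation.
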(event `self.ReceiveBeginPlay`
  ;[1 1 1] Set Location
  (bind _output_get (set `self.InitialLocation` (`SceneComponent.K2_GetComponentLocation` (`self.StaticMesh`))))
  (set `self.EndLocation` (`KismetMathLibrary.MakeVector` (.x _output_get) (.y _output_get) (- (.z _output_get) 2.5))))

(event `self.ReceiveActorBeginOverlap`
  (params (OtherActor :type "Actor Object Reference"))
  (bind _returnvalue (`GameplayStatics.GetActorOfClass` "/Game/Blueprints/BotonClickMismoMomento/BP_Boton2.BP_Boton2_C"))
  (if (`/Game/Blueprints/BotonClickMismoMomento/BP_Boton2.BotonClicked` _returnvalue)
    (`KismetSystemLibrary.PrintString` "Hello"))
  (set `self.BotonClicked` true)
  (bind (_direction _newtrack_0) (`Timeline|Timeline` :!via `PlayFromStart`)
    (:`Update`
      (`SceneComponent.K2_SetWorldLocation` (`self.StaticMesh`) (`KismetMathLibrary.VLerp` (`self.InitialLocation`) (`self.EndLocation`) _newtrack_0) false false))
    (:`Finished`
      (bind (_direction_2 _newtrack_0_2) (`Timeline|Timeline_0` :!via `ReverseFromEnd`)
        (:`Update`
          (`SceneComponent.K2_SetWorldLocation` (`self.StaticMesh`) (`KismetMathLibrary.VLerp` (`self.InitialLocation`) (`self.EndLocation`) _newtrack_0_2) false false))
        (:`Finished`
          (set `self.BotonClicked` false))))))

(event `self.ReceiveActorEndOverlap`
  (params (OtherActor :type "Actor Object Reference")))

(fn `UserConstructionScript`)