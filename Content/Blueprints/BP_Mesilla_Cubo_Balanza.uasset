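; Nightstand Blueprint with a drawer that slides open and a grabbable handle.
; AbrirCajon moves the upper drawer component to a fixed local Y over one second, with debug prints.
; The GrabComponent turns physics simulation off on the handle collision mesh when grabbed and back on when dropped.
; BeginPlay attaches a second upper-drawer component to that handle mesh, snapping location and scale while keeping relative rotation.
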(event `AbrirCajon`
  (bind _v001_mesilla_cajon_cajon_arriba (`self.v001_Mesilla_Cajon_Cajon_Arriba`))
  (bind (_relativelocation_x _relativelocation_y _relativelocation_z) (`KismetMathLibrary.BreakVector` (`SceneComponent.RelativeLocation` _v001_mesilla_cajon_cajon_arriba)))
  (`KismetSystemLibrary.PrintString` "Hello")
  (`KismetSystemLibrary.MoveComponentTo` _v001_mesilla_cajon_cajon_arriba (`KismetMathLibrary.MakeVector` _relativelocation_x 45.0 _relativelocation_z) (struct) false false 1.0)
  (`KismetSystemLibrary.PrintString` "movido"))

(event `self.GrabComponent.OnGrabbed`
  (`PrimitiveComponent.SetSimulatePhysics` (`self.v003_Mesilla_SoloAsa_Collision`) false))

(event `self.GrabComponent.OnDropped`
  (`PrimitiveComponent.SetSimulatePhysics` (`self.v003_Mesilla_SoloAsa_Collision`) true))

(event `self.ReceiveBeginPlay`
  (`SceneComponent.K2_AttachToComponent` (`self.v001_Mesilla_Cajon_Cajon_Arriba1`) (`self.v003_Mesilla_SoloAsa_Collision`) "None" "SnapToTarget" "KeepRelative" "SnapToTarget" true))

(fn `UserConstructionScript`)