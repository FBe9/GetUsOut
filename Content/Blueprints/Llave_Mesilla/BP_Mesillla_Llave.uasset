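; Nightstand lock (Mesilla) that opens its two doors when the matching key actor, BP_Llave_Mesilla, overlaps its box trigger.
; On overlap it disables the key's physics, snaps it to a hardcoded world location and plays a turning sound while a timeline rolls it.
; When the turn finishes, the key is destroyed, an opening sound plays and a second timeline swings both doors by relative yaw.
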(event `self.Box.OnComponentBeginOverlap`
  (params (OverlappedComponent :type "PrimitiveComponent Object Reference") (OtherActor :type "Actor Object Reference") (OtherComp :type "PrimitiveComponent Object Reference") (OtherBodyIndex :type Integer) (bFromSweep :type Boolean) (SweepResult :type "HitResult Structure (by ref)"))
  (bind _asbp_llave_mesilla (cast `/Game/Blueprints/Llave_Mesilla/BP_Llave_Mesilla` OtherActor))
  (`PrimitiveComponent.SetSimulatePhysics` (`/Game/Blueprints/Llave_Mesilla/BP_Llave_Mesilla.StaticMesh` _asbp_llave_mesilla) false)
  (`self.K2_SetActorLocation` _asbp_llave_mesilla (-351.734435 186.723777 51.791432) false false)
  (`GameplayStatics.PlaySound2D` "/Game/Audio/Audio_GirarLlave_Mesilla.Audio_GirarLlave_Mesilla" 1.0 1.0 0.0 null null)
  (bind (_direction _newtrack_0) (`Timeline|Timeline`)
    (:`Update`
      (`self.K2_SetActorRotation` _asbp_llave_mesilla (`KismetMathLibrary.MakeRotator` _newtrack_0) false))
    (:`Finished`
      (`self.K2_DestroyActor` _asbp_llave_mesilla)
      (`GameplayStatics.PlaySound2D` "/Game/Audio/Audio_AbrirPuertas_Mesilla.Audio_AbrirPuertas_Mesilla" 1.0 1.0 0.0 null null)
      (bind (_direction_2 _newtrack_0_2 _newtrack_1) (`Timeline|Timeline_0`)
        (:`Update`
          (`SceneComponent.K2_SetRelativeRotation` (`self.Mueble_Llave_Door_R`) (`KismetMathLibrary.MakeRotator` 0.0 0.0 _newtrack_0_2) false false)
          (`SceneComponent.K2_SetRelativeRotation` (`self.Mueble_Llave_Door_L`) (`KismetMathLibrary.MakeRotator` 0.0 0.0 _newtrack_1) false false))))))

(fn `UserConstructionScript`)