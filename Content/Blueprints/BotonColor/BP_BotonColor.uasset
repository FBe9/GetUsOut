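; Color puzzle button that cycles through four colors when overlapped, as part of a combination checked across the BP_BotonColor instances.
; Each accepted overlap advances ColorId, swaps the BotonDown material, and uses two timelines to press and release BotonTop.
; After the animation it compares the first four GetAllActorsOfClass results to ColorList by index, relying on that array's order.
; A match prints "Hello" and leaves the button locked; otherwise it re-arms.
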(event `self.ReceiveBeginPlay`
  ;[1 1 1] Set Location
  (bind _output_get (set `self.InitialLocation` (`SceneComponent.K2_GetComponentLocation` (`self.BotonTop`))))
  (set `self.EndLocation` (`KismetMathLibrary.MakeVector` (.x _output_get) (.y _output_get) (- (.z _output_get) 2.5)))
  (set `self.ColorId` 1))

(event `self.ReceiveActorBeginOverlap`
  (params (OtherActor :type "Actor Object Reference"))
  (if (not (`self.Clicked`))
    (`/Engine/EditorBlueprintResources/StandardMacros.IncrementInt` (`self.ColorId`)
      (:`  `
        (set `self.Clicked` true)
        (if (== (`self.ColorId`) 5)
          (set `self.ColorId` 1))
        (if (== (`self.ColorId`) 1)
          (`PrimitiveComponent.SetMaterial` (`self.BotonDown`) 0 "/Game/Blueprints/BombaYBoton/MI_Cable_6.MI_Cable_6")
          (bind (_direction _newtrack_0) (`Timeline|Timeline_1` :!via `PlayFromStart` :!label _label)
            (:`Update`
              (`SceneComponent.K2_SetWorldLocation` (`self.BotonTop`) (`KismetMathLibrary.VLerp` (`self.InitialLocation`) (`self.EndLocation`) _newtrack_0) false false))
            (:`Finished`
              (bind (_direction_2 _newtrack_0_2) (`Timeline|Timeline_2` :!via `ReverseFromEnd`)
                (:`Update`
                  (`SceneComponent.K2_SetWorldLocation` (`self.BotonTop`) (`KismetMathLibrary.VLerp` (`self.InitialLocation`) (`self.EndLocation`) _newtrack_0_2) false false))
                (:`Finished`
                  (bind _outactors (`GameplayStatics.GetAllActorsOfClass` "BP_BotonColor_C"))
                  (if (and (== (`/Game/Blueprints/BotonColor/BP_BotonColor.ColorId` (`|GetArrayItem` _outactors)) (`|GetArrayItem` (`self.ColorList`))) (== (`/Game/Blueprints/BotonColor/BP_BotonColor.ColorId` (`|GetArrayItem` _outactors 1)) (`|GetArrayItem` (`self.ColorList`) 1)) (== (`/Game/Blueprints/BotonColor/BP_BotonColor.ColorId` (`|GetArrayItem` _outactors 2)) (`|GetArrayItem` (`self.ColorList`) 2)) (== (`/Game/Blueprints/BotonColor/BP_BotonColor.ColorId` (`|GetArrayItem` _outactors 3)) (`|GetArrayItem` (`self.ColorList`) 3)))
                    (`KismetSystemLibrary.PrintString` "Hello")
                    (else
                      (set `self.Clicked` false)))))))
          (elif (== (`self.ColorId`) 2)
            (`PrimitiveComponent.SetMaterial` (`self.BotonDown`) 0 "/Game/Blueprints/BombaYBoton/MI_Cable_4.MI_Cable_4")
            (goto _label :!via `PlayFromStart`)
            (elif (== (`self.ColorId`) 3)
              (`PrimitiveComponent.SetMaterial` (`self.BotonDown`) 0 "/Game/Blueprints/BombaYBoton/MI_Cable_2.MI_Cable_2")
              (goto _label :!via `PlayFromStart`)
              (elif (== (`self.ColorId`) 4)
                (`PrimitiveComponent.SetMaterial` (`self.BotonDown`) 0 "/Game/Blueprints/BombaYBoton/MI_Cable_1.MI_Cable_1")
                (goto _label :!via `PlayFromStart`)))))))))

(fn `UserConstructionScript`)