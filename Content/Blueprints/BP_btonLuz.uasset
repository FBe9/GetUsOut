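; BP_btonLuz is a light switch that toggles the lamps in the level when an actor overlaps it.
; Each overlap flips its Encendido state and rotates the switch mesh between two pitched positions.
; It then fetches every BP_Lampara actor, inverts each lamp's own Encendido flag and sets its Luz visibility to match, so lamps toggle independently rather than copying the switch's state.
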(event `self.ReceiveActorBeginOverlap`
  (params (OtherActor :type "Actor Object Reference"))
  (bind _interruptor_interruptor_boton (`self.Interruptor_Interruptor_Boton`))
  (bind _output_get (set `self.Encendido` (not (`self.Encendido`))))
  (if _output_get
    (`SceneComponent.K2_SetRelativeRotation` _interruptor_interruptor_boton (struct :`Pitch` 4.883549) false false)
    (else
      (`SceneComponent.K2_SetRelativeRotation` _interruptor_interruptor_boton (struct :`Pitch` -7.0) false false)))
  (bind _outactors (`GameplayStatics.GetAllActorsOfClass` "/Game/Blueprints/BP_Lampara.BP_Lampara_C"))
  (for _array_element _outactors
    (bind _output_get_2 (set `/Game/Blueprints/BP_Lampara.Encendido` (not (`/Game/Blueprints/BP_Lampara.Encendido` _array_element)) _array_element))
    (`SceneComponent.SetVisibility` (`/Game/Blueprints/BP_Lampara.Luz` _array_element) _output_get_2 false)))

(fn `UserConstructionScript`)