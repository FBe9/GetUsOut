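; Keypad safe whose physical buttons sink while their overlap boxes are touched and rise back afterwards, using looped MoveComponentTo steps.
; Fully pressed digits send their component-tag number and position counter to WID_PantallaCajaFuerte; Delete steps back and OK requests a code check.
; Exposed events set the open flag, flash or reset the screen frame color, and open the door.
; OpenDoor also teleports a tagged Grabbable_SmallCube to a hardcoded location.
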(event `self.Box_1.OnComponentEndOverlap`
  (params (OverlappedComponent :type "PrimitiveComponent Object Reference") (OtherActor :type "Actor Object Reference") (OtherComp :type "PrimitiveComponent Object Reference") (OtherBodyIndex :type Integer))
  (bind _boton_1 (`self.Boton_1`))
  (bind (_relativelocation_x _relativelocation_y _relativelocation_z) (`KismetMathLibrary.BreakVector` (`SceneComponent.RelativeLocation` _boton_1)))
  (bind _returnvalue (+ _relativelocation_z (* (`self.VelocHundimiento`) -1.0)))
  ;[1 0.5511 0] Retorna a la posicion inical los botones cuando el objeto deja de estar encima
  (set `self.OverlapBox_1` true)
  (if (`self.OverlapBox_1`) :!label _label
    (if (<= _returnvalue (`self.PosicionInicialBoton`))
      (`KismetSystemLibrary.MoveComponentTo` _boton_1 (`KismetMathLibrary.MakeVector` _relativelocation_x _relativelocation_y _returnvalue) (struct) false false (`self.MovementSeconds`) :!label _label_2)
      (goto _label)
      (else
        (goto _label_2 :!via `Stop`)))))

(event `self.Box_4.OnComponentBeginOverlap`
  (params (OverlappedComponent :type "PrimitiveComponent Object Reference") (OtherActor :type "Actor Object Reference") (OtherComp :type "PrimitiveComponent Object Reference") (OtherBodyIndex :type Integer) (bFromSweep :type Boolean) (SweepResult :type "HitResult Structure (by ref)"))
  (bind _boton_4 (`self.Boton_4`))
  (bind (_relativelocation_x _relativelocation_y _relativelocation_z) (`KismetMathLibrary.BreakVector` (`SceneComponent.RelativeLocation` (`self.Boton_4`))))
  (bind _returnvalue (+ _relativelocation_z (`self.VelocHundimiento`)))
  ;[1 0.5511 0] Cuando se pulse un botón lo mueve se llama al metodo ButtonAnimation pasandole el boton y el numero que tiene
  (set `self.OverlapBox_4` false)
  (if (`self.OverlapBox_4`) :!label _label_3
    _
    (elif (>= _returnvalue (`self.HundimientoMaximo`))
      (`KismetSystemLibrary.MoveComponentTo` _boton_4 (`KismetMathLibrary.MakeVector` _relativelocation_x _relativelocation_y _returnvalue) (struct) false false (`self.MovementSeconds`) :!label _label_4)
      (goto _label_3)
      (else
        (`|ExecutionSequence`
          (:`then_0`
            (`self.ButtonAnimation` _boton_4 (`KismetStringLibrary.Conv_StringToInt` (`KismetStringLibrary.Conv_NameToString` (`|GetArrayItem` (`ActorComponent.ComponentTags` OverlappedComponent))))))
          (:`then_1`
            (goto _label_4 :!via `Stop`)))))))

(event `self.Box_9.OnComponentEndOverlap`
  (params (OverlappedComponent :type "PrimitiveComponent Object Reference") (OtherActor :type "Actor Object Reference") (OtherComp :type "PrimitiveComponent Object Reference") (OtherBodyIndex :type Integer))
  (bind _boton_9 (`self.Boton_9`))
  (bind (_relativelocation_x _relativelocation_y _relativelocation_z) (`KismetMathLibrary.BreakVector` (`SceneComponent.RelativeLocation` _boton_9)))
  (bind _returnvalue (+ _relativelocation_z (* (`self.VelocHundimiento`) -1.0)))
  ;[1 0.5511 0] Retorna a la posicion inical los botones cuando el objeto deja de estar encima
  (set `self.OverlapBox_9` true)
  (if (`self.OverlapBox_9`) :!label _label_5
    (if (<= _returnvalue (`self.PosicionInicialBoton`))
      (`KismetSystemLibrary.MoveComponentTo` _boton_9 (`KismetMathLibrary.MakeVector` _relativelocation_x _relativelocation_y _returnvalue) (struct) false false (`self.MovementSeconds`) :!label _label_6)
      (goto _label_5)
      (else
        (goto _label_6 :!via `Stop`)))))

(event `self.Box_9.OnComponentBeginOverlap`
  (params (OverlappedComponent :type "PrimitiveComponent Object Reference") (OtherActor :type "Actor Object Reference") (OtherComp :type "PrimitiveComponent Object Reference") (OtherBodyIndex :type Integer) (bFromSweep :type Boolean) (SweepResult :type "HitResult Structure (by ref)"))
  (bind _boton_9 (`self.Boton_9`))
  (bind (_relativelocation_x _relativelocation_y _relativelocation_z) (`KismetMathLibrary.BreakVector` (`SceneComponent.RelativeLocation` (`self.Boton_9`))))
  (bind _returnvalue (+ _relativelocation_z (`self.VelocHundimiento`)))
  ;[1 0.5511 0] Cuando se pulse un botón lo mueve se llama al metodo ButtonAnimation pasandole el boton y el numero que tiene
  (set `self.OverlapBox_9` false)
  (if (`self.OverlapBox_9`) :!label _label_7
    _
    (elif (>= _returnvalue (`self.HundimientoMaximo`))
      (`KismetSystemLibrary.MoveComponentTo` _boton_9 (`KismetMathLibrary.MakeVector` _relativelocation_x _relativelocation_y _returnvalue) (struct) false false (`self.MovementSeconds`) :!label _label_8)
      (goto _label_7)
      (else
        (`|ExecutionSequence`
          (:`then_0`
            (`self.ButtonAnimation` _boton_9 (`KismetStringLibrary.Conv_StringToInt` (`KismetStringLibrary.Conv_NameToString` (`|GetArrayItem` (`ActorComponent.ComponentTags` OverlappedComponent))))))
          (:`then_1`
            (goto _label_8 :!via `Stop`)))))))

(event `self.Box_8.OnComponentEndOverlap`
  (params (OverlappedComponent :type "PrimitiveComponent Object Reference") (OtherActor :type "Actor Object Reference") (OtherComp :type "PrimitiveComponent Object Reference") (OtherBodyIndex :type Integer))
  (bind _boton_8 (`self.Boton_8`))
  (bind (_relativelocation_x _relativelocation_y _relativelocation_z) (`KismetMathLibrary.BreakVector` (`SceneComponent.RelativeLocation` _boton_8)))
  (bind _returnvalue (+ _relativelocation_z (* (`self.VelocHundimiento`) -1.0)))
  ;[1 0.5511 0] Retorna a la posicion inical los botones cuando el objeto deja de estar encima
  (set `self.OverlapBox_8` true)
  (if (`self.OverlapBox_8`) :!label _label_9
    (if (<= _returnvalue (`self.PosicionInicialBoton`))
      (`KismetSystemLibrary.MoveComponentTo` _boton_8 (`KismetMathLibrary.MakeVector` _relativelocation_x _relativelocation_y _returnvalue) (struct) false false (`self.MovementSeconds`) :!label _label_10)
      (goto _label_9)
      (else
        (goto _label_10 :!via `Stop`)))))

(event `self.Box_8.OnComponentBeginOverlap`
  (params (OverlappedComponent :type "PrimitiveComponent Object Reference") (OtherActor :type "Actor Object Reference") (OtherComp :type "PrimitiveComponent Object Reference") (OtherBodyIndex :type Integer) (bFromSweep :type Boolean) (SweepResult :type "HitResult Structure (by ref)"))
  (bind _boton_8 (`self.Boton_8`))
  (bind (_relativelocation_x _relativelocation_y _relativelocation_z) (`KismetMathLibrary.BreakVector` (`SceneComponent.RelativeLocation` (`self.Boton_8`))))
  (bind _returnvalue (+ _relativelocation_z (`self.VelocHundimiento`)))
  ;[1 0.5511 0] Cuando se pulse un botón lo mueve se llama al metodo ButtonAnimation pasandole el boton y el numero que tiene
  (set `self.OverlapBox_8` false)
  (if (`self.OverlapBox_8`) :!label _label_11
    _
    (elif (>= _returnvalue (`self.HundimientoMaximo`))
      (`KismetSystemLibrary.MoveComponentTo` _boton_8 (`KismetMathLibrary.MakeVector` _relativelocation_x _relativelocation_y _returnvalue) (struct) false false (`self.MovementSeconds`) :!label _label_12)
      (goto _label_11)
      (else
        (`|ExecutionSequence`
          (:`then_0`
            (`self.ButtonAnimation` _boton_8 (`KismetStringLibrary.Conv_StringToInt` (`KismetStringLibrary.Conv_NameToString` (`|GetArrayItem` (`ActorComponent.ComponentTags` OverlappedComponent))))))
          (:`then_1`
            (goto _label_12 :!via `Stop`)))))))

(event `self.Box_0.OnComponentEndOverlap`
  (params (OverlappedComponent :type "PrimitiveComponent Object Reference") (OtherActor :type "Actor Object Reference") (OtherComp :type "PrimitiveComponent Object Reference") (OtherBodyIndex :type Integer))
  (bind _boton_0 (`self.Boton_0`))
  (bind (_relativelocation_x _relativelocation_y _relativelocation_z) (`KismetMathLibrary.BreakVector` (`SceneComponent.RelativeLocation` _boton_0)))
  (bind _returnvalue (+ _relativelocation_z (* (`self.VelocHundimiento`) -1.0)))
  ;[1 0.5511 0] Retorna a la posicion inical los botones cuando el objeto deja de estar encima
  (set `self.OverlapBox_0` true)
  (if (`self.OverlapBox_0`) :!label _label_13
    (if (<= _returnvalue (`self.PosicionInicialBoton`))
      (`KismetSystemLibrary.MoveComponentTo` _boton_0 (`KismetMathLibrary.MakeVector` _relativelocation_x _relativelocation_y _returnvalue) (struct) false false (`self.MovementSeconds`) :!label _label_14)
      (goto _label_13)
      (else
        (goto _label_14 :!via `Stop`)))))

(event `self.Box_3.OnComponentBeginOverlap`
  (params (OverlappedComponent :type "PrimitiveComponent Object Reference") (OtherActor :type "Actor Object Reference") (OtherComp :type "PrimitiveComponent Object Reference") (OtherBodyIndex :type Integer) (bFromSweep :type Boolean) (SweepResult :type "HitResult Structure (by ref)"))
  (bind _boton_3 (`self.Boton_3`))
  (bind (_relativelocation_x _relativelocation_y _relativelocation_z) (`KismetMathLibrary.BreakVector` (`SceneComponent.RelativeLocation` (`self.Boton_3`))))
  (bind _returnvalue (+ _relativelocation_z (`self.VelocHundimiento`)))
  ;[1 0.5511 0] Cuando se pulse un botón lo mueve se llama al metodo ButtonAnimation pasandole el boton y el numero que tiene
  (set `self.OverlapBox_3` false)
  (if (`self.OverlapBox_3`) :!label _label_15
    _
    (elif (>= _returnvalue (`self.HundimientoMaximo`))
      (`KismetSystemLibrary.MoveComponentTo` _boton_3 (`KismetMathLibrary.MakeVector` _relativelocation_x _relativelocation_y _returnvalue) (struct) false false (`self.MovementSeconds`) :!label _label_16)
      (goto _label_15)
      (else
        (`|ExecutionSequence`
          (:`then_0`
            (`self.ButtonAnimation` _boton_3 (`KismetStringLibrary.Conv_StringToInt` (`KismetStringLibrary.Conv_NameToString` (`|GetArrayItem` (`ActorComponent.ComponentTags` OverlappedComponent))))))
          (:`then_1`
            (goto _label_16 :!via `Stop`)))))))

(event `ButtonReturnPosition`
  (params (Button :type "StaticMeshComponent Object Reference") (Box :type "BoxComponent Object Reference") (BoxOverlap :type Boolean))
  ;[1 0.5511 0] Retorna a la posicion inical los botones cuando el objeto deja de estar encima
)

(event `self.Box_7.OnComponentEndOverlap`
  (params (OverlappedComponent :type "PrimitiveComponent Object Reference") (OtherActor :type "Actor Object Reference") (OtherComp :type "PrimitiveComponent Object Reference") (OtherBodyIndex :type Integer))
  (bind _boton_7 (`self.Boton_7`))
  (bind (_relativelocation_x _relativelocation_y _relativelocation_z) (`KismetMathLibrary.BreakVector` (`SceneComponent.RelativeLocation` _boton_7)))
  (bind _returnvalue (+ _relativelocation_z (* (`self.VelocHundimiento`) -1.0)))
  ;[1 0.5511 0] Retorna a la posicion inical los botones cuando el objeto deja de estar encima
  (set `self.OverlapBox_7` true)
  (if (`self.OverlapBox_7`) :!label _label_17
    (if (<= _returnvalue (`self.PosicionInicialBoton`))
      (`KismetSystemLibrary.MoveComponentTo` _boton_7 (`KismetMathLibrary.MakeVector` _relativelocation_x _relativelocation_y _returnvalue) (struct) false false (`self.MovementSeconds`) :!label _label_18)
      (goto _label_17)
      (else
        (goto _label_18 :!via `Stop`)))))

(event `self.Box_2.OnComponentBeginOverlap`
  (params (OverlappedComponent :type "PrimitiveComponent Object Reference") (OtherActor :type "Actor Object Reference") (OtherComp :type "PrimitiveComponent Object Reference") (OtherBodyIndex :type Integer) (bFromSweep :type Boolean) (SweepResult :type "HitResult Structure (by ref)"))
  (bind _boton_2 (`self.Boton_2`))
  (bind (_relativelocation_x _relativelocation_y _relativelocation_z) (`KismetMathLibrary.BreakVector` (`SceneComponent.RelativeLocation` (`self.Boton_2`))))
  (bind _returnvalue (+ _relativelocation_z (`self.VelocHundimiento`)))
  ;[1 0.5511 0] Cuando se pulse un botón lo mueve se llama al metodo ButtonAnimation pasandole el boton y el numero que tiene
  (set `self.OverlapBox_2` false)
  (if (`self.OverlapBox_2`) :!label _label_19
    _
    (elif (>= _returnvalue (`self.HundimientoMaximo`))
      (`KismetSystemLibrary.MoveComponentTo` _boton_2 (`KismetMathLibrary.MakeVector` _relativelocation_x _relativelocation_y _returnvalue) (struct) false false (`self.MovementSeconds`) :!label _label_20)
      (goto _label_19)
      (else
        (`|ExecutionSequence`
          (:`then_0`
            (`self.ButtonAnimation` _boton_2 (`KismetStringLibrary.Conv_StringToInt` (`KismetStringLibrary.Conv_NameToString` (`|GetArrayItem` (`ActorComponent.ComponentTags` OverlappedComponent))))))
          (:`then_1`
            (goto _label_20 :!via `Stop`)))))))

(event `self.Box_ok.OnComponentEndOverlap`
  (params (OverlappedComponent :type "PrimitiveComponent Object Reference") (OtherActor :type "Actor Object Reference") (OtherComp :type "PrimitiveComponent Object Reference") (OtherBodyIndex :type Integer))
  (bind _boton_ok (`self.Boton_OK`))
  (bind (_relativelocation_x _relativelocation_y _relativelocation_z) (`KismetMathLibrary.BreakVector` (`SceneComponent.RelativeLocation` _boton_ok)))
  (bind _returnvalue (+ _relativelocation_z (* (`self.VelocHundimiento`) -1.0)))
  ;[1 0.5511 0] Retorna a la posicion inical los botones cuando el objeto deja de estar encima
  (set `self.OverlapBox_Ok` true)
  (if (`self.OverlapBox_Ok`) :!label _label_21
    (if (<= _returnvalue (`self.PosicionInicialBoton`))
      (`KismetSystemLibrary.MoveComponentTo` _boton_ok (`KismetMathLibrary.MakeVector` _relativelocation_x _relativelocation_y _returnvalue) (struct) false false (`self.MovementSeconds`) :!label _label_22)
      (goto _label_21)
      (else
        (goto _label_22 :!via `Stop`)))))

(event `self.Box_7.OnComponentBeginOverlap`
  (params (OverlappedComponent :type "PrimitiveComponent Object Reference") (OtherActor :type "Actor Object Reference") (OtherComp :type "PrimitiveComponent Object Reference") (OtherBodyIndex :type Integer) (bFromSweep :type Boolean) (SweepResult :type "HitResult Structure (by ref)"))
  (bind _boton_7 (`self.Boton_7`))
  (bind (_relativelocation_x _relativelocation_y _relativelocation_z) (`KismetMathLibrary.BreakVector` (`SceneComponent.RelativeLocation` (`self.Boton_7`))))
  (bind _returnvalue (+ _relativelocation_z (`self.VelocHundimiento`)))
  ;[1 0.5511 0] Cuando se pulse un botón lo mueve se llama al metodo ButtonAnimation pasandole el boton y el numero que tiene
  (set `self.OverlapBox_7` false)
  (if (`self.OverlapBox_7`) :!label _label_23
    _
    (elif (>= _returnvalue (`self.HundimientoMaximo`))
      (`KismetSystemLibrary.MoveComponentTo` _boton_7 (`KismetMathLibrary.MakeVector` _relativelocation_x _relativelocation_y _returnvalue) (struct) false false (`self.MovementSeconds`) :!label _label_24)
      (goto _label_23)
      (else
        (`|ExecutionSequence`
          (:`then_0`
            (`self.ButtonAnimation` _boton_7 (`KismetStringLibrary.Conv_StringToInt` (`KismetStringLibrary.Conv_NameToString` (`|GetArrayItem` (`ActorComponent.ComponentTags` OverlappedComponent))))))
          (:`then_1`
            (goto _label_24 :!via `Stop`)))))))

(event `self.Box_6.OnComponentEndOverlap`
  (params (OverlappedComponent :type "PrimitiveComponent Object Reference") (OtherActor :type "Actor Object Reference") (OtherComp :type "PrimitiveComponent Object Reference") (OtherBodyIndex :type Integer))
  (bind _boton_6 (`self.Boton_6`))
  (bind (_relativelocation_x _relativelocation_y _relativelocation_z) (`KismetMathLibrary.BreakVector` (`SceneComponent.RelativeLocation` _boton_6)))
  (bind _returnvalue (+ _relativelocation_z (* (`self.VelocHundimiento`) -1.0)))
  ;[1 0.5511 0] Retorna a la posicion inical los botones cuando el objeto deja de estar encima
  (set `self.OverlapBox_6` true)
  (if (`self.OverlapBox_6`) :!label _label_25
    (if (<= _returnvalue (`self.PosicionInicialBoton`))
      (`KismetSystemLibrary.MoveComponentTo` _boton_6 (`KismetMathLibrary.MakeVector` _relativelocation_x _relativelocation_y _returnvalue) (struct) false false (`self.MovementSeconds`) :!label _label_26)
      (goto _label_25)
      (else
        (goto _label_26 :!via `Stop`)))))

(event `self.Box_delete.OnComponentEndOverlap`
  (params (OverlappedComponent :type "PrimitiveComponent Object Reference") (OtherActor :type "Actor Object Reference") (OtherComp :type "PrimitiveComponent Object Reference") (OtherBodyIndex :type Integer))
  (bind _boton_delete (`self.Boton_Delete`))
  (bind (_relativelocation_x _relativelocation_y _relativelocation_z) (`KismetMathLibrary.BreakVector` (`SceneComponent.RelativeLocation` _boton_delete)))
  (bind _returnvalue (+ _relativelocation_z (* (`self.VelocHundimiento`) -1.0)))
  ;[1 0.5511 0] Retorna a la posicion inical los botones cuando el objeto deja de estar encima
  (set `self.OverlapBox_Delete` true)
  (if (`self.OverlapBox_Delete`) :!label _label_27
    (if (<= _returnvalue (`self.PosicionInicialBoton`))
      (`KismetSystemLibrary.MoveComponentTo` _boton_delete (`KismetMathLibrary.MakeVector` _relativelocation_x _relativelocation_y _returnvalue) (struct) false false (`self.MovementSeconds`) :!label _label_28)
      (goto _label_27)
      (else
        (goto _label_28 :!via `Stop`)))))

(event `self.Box_1.OnComponentBeginOverlap`
  (params (OverlappedComponent :type "PrimitiveComponent Object Reference") (OtherActor :type "Actor Object Reference") (OtherComp :type "PrimitiveComponent Object Reference") (OtherBodyIndex :type Integer) (bFromSweep :type Boolean) (SweepResult :type "HitResult Structure (by ref)"))
  (bind _boton_1 (`self.Boton_1`))
  (bind (_relativelocation_x _relativelocation_y _relativelocation_z) (`KismetMathLibrary.BreakVector` (`SceneComponent.RelativeLocation` (`self.Boton_1`))))
  (bind _returnvalue (+ _relativelocation_z (`self.VelocHundimiento`)))
  ;[1 0.5511 0] Cuando se pulse un botón lo mueve se llama al metodo ButtonAnimation pasandole el boton y el numero que tiene
  (set `self.OverlapBox_1` false)
  (if (`self.OverlapBox_1`) :!label _label_29
    _
    (elif (>= _returnvalue (`self.HundimientoMaximo`))
      (`KismetSystemLibrary.MoveComponentTo` _boton_1 (`KismetMathLibrary.MakeVector` _relativelocation_x _relativelocation_y _returnvalue) (struct) false false (`self.MovementSeconds`) :!label _label_30)
      (goto _label_29)
      (else
        (`|ExecutionSequence`
          (:`then_0`
            (`self.ButtonAnimation` _boton_1 (`KismetStringLibrary.Conv_StringToInt` (`KismetStringLibrary.Conv_NameToString` (`|GetArrayItem` (`ActorComponent.ComponentTags` OverlappedComponent))))))
          (:`then_1`
            (goto _label_30 :!via `Stop`)))))))

(event `self.Box_6.OnComponentBeginOverlap`
  (params (OverlappedComponent :type "PrimitiveComponent Object Reference") (OtherActor :type "Actor Object Reference") (OtherComp :type "PrimitiveComponent Object Reference") (OtherBodyIndex :type Integer) (bFromSweep :type Boolean) (SweepResult :type "HitResult Structure (by ref)"))
  (bind _boton_6 (`self.Boton_6`))
  (bind (_relativelocation_x _relativelocation_y _relativelocation_z) (`KismetMathLibrary.BreakVector` (`SceneComponent.RelativeLocation` (`self.Boton_6`))))
  (bind _returnvalue (+ _relativelocation_z (`self.VelocHundimiento`)))
  ;[1 0.5511 0] Cuando se pulse un botón lo mueve se llama al metodo ButtonAnimation pasandole el boton y el numero que tiene
  (set `self.OverlapBox_6` false)
  (if (`self.OverlapBox_6`) :!label _label_31
    _
    (elif (>= _returnvalue (`self.HundimientoMaximo`))
      (`KismetSystemLibrary.MoveComponentTo` _boton_6 (`KismetMathLibrary.MakeVector` _relativelocation_x _relativelocation_y _returnvalue) (struct) false false (`self.MovementSeconds`) :!label _label_32)
      (goto _label_31)
      (else
        (`|ExecutionSequence`
          (:`then_0`
            (`self.ButtonAnimation` _boton_6 (`KismetStringLibrary.Conv_StringToInt` (`KismetStringLibrary.Conv_NameToString` (`|GetArrayItem` (`ActorComponent.ComponentTags` OverlappedComponent))))))
          (:`then_1`
            (goto _label_32 :!via `Stop`)))))))

(event `self.Box_5.OnComponentEndOverlap`
  (params (OverlappedComponent :type "PrimitiveComponent Object Reference") (OtherActor :type "Actor Object Reference") (OtherComp :type "PrimitiveComponent Object Reference") (OtherBodyIndex :type Integer))
  (bind _boton_5 (`self.Boton_5`))
  (bind (_relativelocation_x _relativelocation_y _relativelocation_z) (`KismetMathLibrary.BreakVector` (`SceneComponent.RelativeLocation` _boton_5)))
  (bind _returnvalue (+ _relativelocation_z (* (`self.VelocHundimiento`) -1.0)))
  ;[1 0.5511 0] Retorna a la posicion inical los botones cuando el objeto deja de estar encima
  (set `self.OverlapBox_5` true)
  (if (`self.OverlapBox_5`) :!label _label_33
    (if (<= _returnvalue (`self.PosicionInicialBoton`))
      (`KismetSystemLibrary.MoveComponentTo` _boton_5 (`KismetMathLibrary.MakeVector` _relativelocation_x _relativelocation_y _returnvalue) (struct) false false (`self.MovementSeconds`) :!label _label_34)
      (goto _label_33)
      (else
        (goto _label_34 :!via `Stop`)))))

(event `self.Box_3.OnComponentEndOverlap`
  (params (OverlappedComponent :type "PrimitiveComponent Object Reference") (OtherActor :type "Actor Object Reference") (OtherComp :type "PrimitiveComponent Object Reference") (OtherBodyIndex :type Integer))
  (bind _boton_3 (`self.Boton_3`))
  (bind (_relativelocation_x _relativelocation_y _relativelocation_z) (`KismetMathLibrary.BreakVector` (`SceneComponent.RelativeLocation` _boton_3)))
  (bind _returnvalue (+ _relativelocation_z (* (`self.VelocHundimiento`) -1.0)))
  ;[1 0.5511 0] Retorna a la posicion inical los botones cuando el objeto deja de estar encima
  (set `self.OverlapBox_3` true)
  (if (`self.OverlapBox_3`) :!label _label_35
    (if (<= _returnvalue (`self.PosicionInicialBoton`))
      (`KismetSystemLibrary.MoveComponentTo` _boton_3 (`KismetMathLibrary.MakeVector` _relativelocation_x _relativelocation_y _returnvalue) (struct) false false (`self.MovementSeconds`) :!label _label_36)
      (goto _label_35)
      (else
        (goto _label_36 :!via `Stop`)))))

(event `self.Box_0.OnComponentBeginOverlap`
  (params (OverlappedComponent :type "PrimitiveComponent Object Reference") (OtherActor :type "Actor Object Reference") (OtherComp :type "PrimitiveComponent Object Reference") (OtherBodyIndex :type Integer) (bFromSweep :type Boolean) (SweepResult :type "HitResult Structure (by ref)"))
  (bind _boton_0 (`self.Boton_0`))
  (bind (_relativelocation_x _relativelocation_y _relativelocation_z) (`KismetMathLibrary.BreakVector` (`SceneComponent.RelativeLocation` (`self.Boton_0`))))
  (bind _returnvalue (+ _relativelocation_z (`self.VelocHundimiento`)))
  ;[1 0.5511 0] Cuando se pulse un botón lo mueve se llama al metodo ButtonAnimation pasandole el boton y el numero que tiene
  (set `self.OverlapBox_0` false)
  (if (`self.OverlapBox_0`) :!label _label_37
    _
    (elif (>= _returnvalue (`self.HundimientoMaximo`))
      (`KismetSystemLibrary.MoveComponentTo` _boton_0 (`KismetMathLibrary.MakeVector` _relativelocation_x _relativelocation_y _returnvalue) (struct) false false (`self.MovementSeconds`) :!label _label_38)
      (goto _label_37)
      (else
        (`|ExecutionSequence`
          (:`then_0`
            (`self.ButtonAnimation` _boton_0 (`KismetStringLibrary.Conv_StringToInt` (`KismetStringLibrary.Conv_NameToString` (`|GetArrayItem` (`ActorComponent.ComponentTags` OverlappedComponent))))))
          (:`then_1`
            (goto _label_38 :!via `Stop`)))))))

(event `self.Box_5.OnComponentBeginOverlap`
  (params (OverlappedComponent :type "PrimitiveComponent Object Reference") (OtherActor :type "Actor Object Reference") (OtherComp :type "PrimitiveComponent Object Reference") (OtherBodyIndex :type Integer) (bFromSweep :type Boolean) (SweepResult :type "HitResult Structure (by ref)"))
  (bind _boton_5 (`self.Boton_5`))
  (bind (_relativelocation_x _relativelocation_y _relativelocation_z) (`KismetMathLibrary.BreakVector` (`SceneComponent.RelativeLocation` (`self.Boton_5`))))
  (bind _returnvalue (+ _relativelocation_z (`self.VelocHundimiento`)))
  ;[1 0.5511 0] Cuando se pulse un botón lo mueve se llama al metodo ButtonAnimation pasandole el boton y el numero que tiene
  (set `self.OverlapBox_5` false)
  (if (`self.OverlapBox_5`) :!label _label_39
    _
    (elif (>= _returnvalue (`self.HundimientoMaximo`))
      (`KismetSystemLibrary.MoveComponentTo` _boton_5 (`KismetMathLibrary.MakeVector` _relativelocation_x _relativelocation_y _returnvalue) (struct) false false (`self.MovementSeconds`) :!label _label_40)
      (goto _label_39)
      (else
        (`|ExecutionSequence`
          (:`then_0`
            (`self.ButtonAnimation` _boton_5 (`KismetStringLibrary.Conv_StringToInt` (`KismetStringLibrary.Conv_NameToString` (`|GetArrayItem` (`ActorComponent.ComponentTags` OverlappedComponent))))))
          (:`then_1`
            (goto _label_40 :!via `Stop`)))))))

(event `self.Box_4.OnComponentEndOverlap`
  (params (OverlappedComponent :type "PrimitiveComponent Object Reference") (OtherActor :type "Actor Object Reference") (OtherComp :type "PrimitiveComponent Object Reference") (OtherBodyIndex :type Integer))
  (bind _boton_4 (`self.Boton_4`))
  (bind (_relativelocation_x _relativelocation_y _relativelocation_z) (`KismetMathLibrary.BreakVector` (`SceneComponent.RelativeLocation` _boton_4)))
  (bind _returnvalue (+ _relativelocation_z (* (`self.VelocHundimiento`) -1.0)))
  ;[1 0.5511 0] Retorna a la posicion inical los botones cuando el objeto deja de estar encima
  (set `self.OverlapBox_4` true)
  (if (`self.OverlapBox_4`) :!label _label_41
    (if (<= _returnvalue (`self.PosicionInicialBoton`))
      (`KismetSystemLibrary.MoveComponentTo` _boton_4 (`KismetMathLibrary.MakeVector` _relativelocation_x _relativelocation_y _returnvalue) (struct) false false (`self.MovementSeconds`) :!label _label_42)
      (goto _label_41)
      (else
        (goto _label_42 :!via `Stop`)))))

(event `self.Box_2.OnComponentEndOverlap`
  (params (OverlappedComponent :type "PrimitiveComponent Object Reference") (OtherActor :type "Actor Object Reference") (OtherComp :type "PrimitiveComponent Object Reference") (OtherBodyIndex :type Integer))
  (bind _boton_2 (`self.Boton_2`))
  (bind (_relativelocation_x _relativelocation_y _relativelocation_z) (`KismetMathLibrary.BreakVector` (`SceneComponent.RelativeLocation` _boton_2)))
  (bind _returnvalue (+ _relativelocation_z (* (`self.VelocHundimiento`) -1.0)))
  ;[1 0.5511 0] Retorna a la posicion inical los botones cuando el objeto deja de estar encima
  (set `self.OverlapBox_2` true)
  (if (`self.OverlapBox_2`) :!label _label_43
    (if (<= _returnvalue (`self.PosicionInicialBoton`))
      (`KismetSystemLibrary.MoveComponentTo` _boton_2 (`KismetMathLibrary.MakeVector` _relativelocation_x _relativelocation_y _returnvalue) (struct) false false (`self.MovementSeconds`) :!label _label_44)
      (goto _label_43)
      (else
        (goto _label_44 :!via `Stop`)))))

(event `self.Box_ok.OnComponentBeginOverlap`
  (params (OverlappedComponent :type "PrimitiveComponent Object Reference") (OtherActor :type "Actor Object Reference") (OtherComp :type "PrimitiveComponent Object Reference") (OtherBodyIndex :type Integer) (bFromSweep :type Boolean) (SweepResult :type "HitResult Structure (by ref)"))
  (bind _open_ (`self.Open?`))
  (bind _boton_ok (`self.Boton_OK`))
  (bind (_relativelocation_x _relativelocation_y _relativelocation_z) (`KismetMathLibrary.BreakVector` (`SceneComponent.RelativeLocation` _boton_ok)))
  (bind _returnvalue (+ _relativelocation_z (`self.VelocHundimiento`)))
  ;[1 0.5342 0] Cuando se pulsa el boton ok(la colision) mueve el boton hacia atras y llama al evento CheckCorrectCode del WID_PantallaCajaFuerte
  (set `self.OverlapBox_Ok` false)
  (if (`self.OverlapBox_Ok`) :!label _label_45
    _
    (elif (>= _returnvalue (`self.HundimientoMaximo`))
      (`KismetSystemLibrary.MoveComponentTo` _boton_ok (`KismetMathLibrary.MakeVector` _relativelocation_x _relativelocation_y _returnvalue) (struct) false false (`self.MovementSeconds`) :!label _label_46)
      (goto _label_45)
      (else
        (`|ExecutionSequence`
          (:`then_0`
            (goto _label_46 :!via `Stop`))
          (:`then_1`
            (bind _aswid_pantalla_caja_fuerte (cast `/Game/Widgets/WID_PantallaCajaFuerte` (`WidgetComponent.GetWidget` (`self.Widget`))))
            (`KismetSystemLibrary.PrintString` (`KismetStringLibrary.Conv_BoolToString` _open_) true true (struct :`R` 1.0 :`G` 0.899021 :`B` 0.031194 :`A` 1.0) 5.0)
            (if (not _open_)
              (`/Game/Widgets/WID_PantallaCajaFuerte.CheckCorrectCode` _aswid_pantalla_caja_fuerte))))))))

(event `ButtonAnimation`
  (params (BotonPresionado :type "StaticMeshComponent Object Reference") (Numero :type Integer))
  (bind _contador (`self.Contador`))
  ;[1 0.2217 0.09193] Mueve el boton correspondiente y llama al metodo ChangeValue del WID_PantallaCajaFuerte
  (`GameplayStatics.PlaySound2D` "/Engine/EditorSounds/GamePreview/StartPlayInEditor.StartPlayInEditor" 1.0 1.0 0.0 null null)
  (bind _aswid_pantalla_caja_fuerte (cast `/Game/Widgets/WID_PantallaCajaFuerte` (`WidgetComponent.GetWidget` (`self.Widget`))))
  (`/Game/Widgets/WID_PantallaCajaFuerte.ChangeValue` _aswid_pantalla_caja_fuerte Numero _contador)
  (if (not (== _contador 4))
    (`/Engine/EditorBlueprintResources/StandardMacros.IncrementInt` _contador)))

(event `self.Box_delete.OnComponentBeginOverlap`
  (params (OverlappedComponent :type "PrimitiveComponent Object Reference") (OtherActor :type "Actor Object Reference") (OtherComp :type "PrimitiveComponent Object Reference") (OtherBodyIndex :type Integer) (bFromSweep :type Boolean) (SweepResult :type "HitResult Structure (by ref)"))
  (bind _contador (`self.Contador`))
  (bind _boton_delete (`self.Boton_Delete`))
  (bind (_relativelocation_x _relativelocation_y _relativelocation_z) (`KismetMathLibrary.BreakVector` (`SceneComponent.RelativeLocation` _boton_delete)))
  (bind _returnvalue (+ _relativelocation_z (`self.VelocHundimiento`)))
  ;[1 0.5342 0] Cuando se pulsa el boton delete(la colision) mueve el boton hacia atras y llama al evento Reset del WID_PantallaCajaFuerte
  (set `self.OverlapBox_Delete` false)
  (if (`self.OverlapBox_Delete`) :!label _label_47
    _
    (elif (>= _returnvalue (`self.HundimientoMaximo`))
      (`KismetSystemLibrary.MoveComponentTo` _boton_delete (`KismetMathLibrary.MakeVector` _relativelocation_x _relativelocation_y _returnvalue) (struct) false false (`self.MovementSeconds`) :!label _label_48)
      (goto _label_47)
      (else
        (`|ExecutionSequence`
          (:`then_0`
            (bind _aswid_pantalla_caja_fuerte (cast `/Game/Widgets/WID_PantallaCajaFuerte` (`WidgetComponent.GetWidget` (`self.Widget`))))
            (`GameplayStatics.PlaySound2D` "/Engine/EditorSounds/GamePreview/EndPlayInEditor_Cue.EndPlayInEditor_Cue" 1.0 1.0 0.0 null null)
            (if (not (== _contador 0))
              (bind _result (`/Engine/EditorBlueprintResources/StandardMacros.DecrementInt` _contador)
                (:`  `
                  (`/Game/Widgets/WID_PantallaCajaFuerte.Reset` _aswid_pantalla_caja_fuerte _result)))))
          (:`then_1`
            (goto _label_48 :!via `Stop`)))))))

(event `SetOpen`
  ;[1 0.1885 0.219] Pone la variable Open? en true y añade un sonido al boton
  (set `self.Open?` true)
  (`GameplayStatics.PlaySound2D` "/Engine/EngineSounds/1kSineTonePing.1kSineTonePing" 1.0 1.0 0.0 null null))

(event `OpenDoor`
  (bind _cajafuerte_puerta (`self.CajaFuerte_Puerta`))
  (bind _relativelocation (`SceneComponent.RelativeLocation` _cajafuerte_puerta))
  ;[1 0.212 0.202] Abre la puerta, cambia el material de la pantalla por uno verde y  hace sonar un sonido
  (bind _outactors (`GameplayStatics.GetAllActorsOfClassWithTag` "/Game/VRTemplate/Blueprints/Grabbable_SmallCube.Grabbable_SmallCube_C" "2"))
  (bind _output (`|GetArrayItem` _outactors))
  (`KismetSystemLibrary.PrintString` (`KismetSystemLibrary.GetDisplayName` _output) true true (struct :`R` 1.0 :`B` 0.112175 :`A` 1.0) 50.0)
  (bind _returnvalue (`self.K2_TeleportTo` :`self` _output :`DestLocation` (350.0 -144.0 136.486855)))
  (`KismetSystemLibrary.PrintString` (`KismetStringLibrary.Conv_BoolToString` _returnvalue) true true (struct :`R` 0.147643 :`G` 1.0 :`B` 0.053401 :`A` 1.0) 50.0)
  (`PrimitiveComponent.SetMaterial` (`self.CajaFuerte_Pantalla`) 1 "/Game/VRTemplate/Materials/M_LeftEyeGreen_RightEyeRed.M_LeftEyeGreen_RightEyeRed")
  (`GameplayStatics.PlaySoundAtLocation` "/Engine/EditorSounds/Notifications/CompileFailed_Cue.CompileFailed_Cue" _relativelocation (struct) 1.0 1.0 0.0 null null null null)
  (`KismetSystemLibrary.Delay` 2.0)
  (`KismetSystemLibrary.MoveComponentTo` _cajafuerte_puerta _relativelocation (struct :`Pitch` 130.0) false false 5.0)
  (`PrimitiveComponent.SetSimulatePhysics` (`self.CajaFuerte_Puerta`) false))

(event `ResetColor`
  ;[1 0.1885 0.219] Resetea el color del marco y setea el contador a 0
  (`PrimitiveComponent.SetMaterial` (`self.CajaFuerte_Pantalla`) 2 "/Game/LevelPrototyping/Materials/MI_Solid_Blue.MI_Solid_Blue")
  (set `self.Contador` 0))

(event `self.ReceiveBeginPlay`
  (bind _cajafuerte_pantalla (`self.CajaFuerte_Pantalla`))
  (`PrimitiveComponent.SetMaterial` _cajafuerte_pantalla 1 "/Engine/BufferVisualization/Anisotropy.Anisotropy")
  (`PrimitiveComponent.SetMaterial` _cajafuerte_pantalla 2 "/Game/LevelPrototyping/Materials/MI_Solid_Blue.MI_Solid_Blue" :!label _label_49))

(event `SetErrorColor`
  ;[1 0.2135 0.2392] Pone color rojo cuando se introduce un codigo incorrecto
  (`GameplayStatics.PlaySound2D` "/Engine/EditorSounds/Notifications/CompileFailed.CompileFailed" 1.0 1.0 0.0 null null)
  (`PrimitiveComponent.SetMaterial` (`self.CajaFuerte_Pantalla`) 2 "/Engine/VREditor/BasicMeshes/MI_Cube_03.MI_Cube_03")
  (`KismetSystemLibrary.Delay` 0.3)
  (goto _label_49))

(fn `UserConstructionScript`)