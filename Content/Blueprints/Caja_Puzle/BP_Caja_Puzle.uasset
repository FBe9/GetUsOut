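; Puzzle box with a 3x3 grid of trigger slots that slides open a drawer holding a key once all nine cubes are correctly placed.
; Each slot accepts a BP_Cubo_Puzle with near-zero rotation and two matching tags, snaps it into place and sets a flag, cleared on end overlap.
; When all flags are set, AbrirCajon opens the drawer once and restores query collision on the tagged key, set physics-only at BeginPlay.
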(event `self.ReceiveBeginPlay`
  ;[1 1 1] Localizar llave y guardar su info para poder gestionar sus collisiones
  (bind _outactors (`GameplayStatics.GetAllActorsOfClassWithTag` "/Game/Blueprints/Llave_Mesilla/BP_Llave_Mesilla.BP_Llave_Mesilla_C" "llaveU"))
  (bind _output_get (set `self.llave` (`|GetArrayItem` _outactors)))
  (`PrimitiveComponent.SetCollisionEnabled` (`/Game/Blueprints/Llave_Mesilla/BP_Llave_Mesilla.StaticMesh` _output_get) "PhysicsOnly"))

(event `AbrirCajon`
  ;[1 1 1] En el caso de que todos los cubos esten colocados en su sitio se abre el cajón
  (if (and (`self.booBox1-1`) (`self.booBox1-2`) (`self.booBox1-3`) (`self.booBox2-1`) (`self.booBox2-2`) (`self.booBox2-3`) (`self.booBox3-1`) (`self.booBox3-2`) (`self.booBox3-3`))
    (`KismetSystemLibrary.PrintString` "Cajón Abierto")
    (if (not (`self.booAbierto`))
      (set `self.booAbierto` true)
      (`GameplayStatics.PlaySound2D` "/Game/Audio/Audio_AbrirCajon_Caja_Puzle.Audio_AbrirCajon_Caja_Puzle" 1.0 1.0 0.0 null null)
      (`KismetSystemLibrary.MoveComponentTo` (`self.StaticMesh1`) (-5.9 0.0 0.0) (struct) false false 0.9)
      (`PrimitiveComponent.SetCollisionEnabled` (`/Game/Blueprints/Llave_Mesilla/BP_Llave_Mesilla.StaticMesh` (`self.llave`)) "QueryAndPhysics"))))

(event `self.Box1-3.OnComponentEndOverlap`
  (params (OverlappedComponent :type "PrimitiveComponent Object Reference") (OtherActor :type "Actor Object Reference") (OtherComp :type "PrimitiveComponent Object Reference") (OtherBodyIndex :type Integer))
  ;[1 1 1] Box1-3 | Comprobación de el cubo que tiene colocado
  (cast `/Game/Blueprints/Caja_Puzle/BP_Cubo_Puzle` OtherActor)
  (set `self.booBox1-3` false))

(event `self.Box1-1.OnComponentEndOverlap`
  (params (OverlappedComponent :type "PrimitiveComponent Object Reference") (OtherActor :type "Actor Object Reference") (OtherComp :type "PrimitiveComponent Object Reference") (OtherBodyIndex :type Integer))
  ;[1 1 1] Box1-1 | Comprobación de el cubo que tiene colocado
  (cast `/Game/Blueprints/Caja_Puzle/BP_Cubo_Puzle` OtherActor)
  (set `self.booBox1-1` false))

(event `self.Box1-2.OnComponentEndOverlap`
  (params (OverlappedComponent :type "PrimitiveComponent Object Reference") (OtherActor :type "Actor Object Reference") (OtherComp :type "PrimitiveComponent Object Reference") (OtherBodyIndex :type Integer))
  ;[1 1 1] Box1-2 | Comprobación de el cubo que tiene colocado
  (cast `/Game/Blueprints/Caja_Puzle/BP_Cubo_Puzle` OtherActor)
  (set `self.booBox1-2` false))

(event `self.Box1-1.OnComponentBeginOverlap`
  (params (OverlappedComponent :type "PrimitiveComponent Object Reference") (OtherActor :type "Actor Object Reference") (OtherComp :type "PrimitiveComponent Object Reference") (OtherBodyIndex :type Integer) (bFromSweep :type Boolean) (SweepResult :type "HitResult Structure (by ref)"))
  ;[1 1 1] Box1-1 | Comprobación de el cubo que tiene colocado
  (bind _asbp_cubo_puzle (cast `/Game/Blueprints/Caja_Puzle/BP_Cubo_Puzle` OtherActor))
  (bind _tags (`Actor.Tags` _asbp_cubo_puzle))
  (if (and (== (`self.K2_GetActorRotation` _asbp_cubo_puzle) (struct) :`ErrorTolerance` 45.0) (== (`|GetArrayItem` (`ActorComponent.ComponentTags` (`self.Box1-1`))) (`|GetArrayItem` _tags)) (== (`|GetArrayItem` _tags 1) (`|GetArrayItem` (`ActorComponent.ComponentTags` (`self.Box1-1`)) 1)))
    (`KismetSystemLibrary.PrintString` "BIEEN")
    (set `self.booBox1-1` true)
    (`self.K2_SetActorLocation` _asbp_cubo_puzle (`KismetMathLibrary.MakeVector` (`self.row1_X`) (`self.column1_Y`) (`self.zValue`)) false false)
    (`self.AbrirCajon`)
    (else
      (`KismetSystemLibrary.PrintString` "MAAL")
      (set `self.booBox1-1` false))))

(event `self.Box1-2.OnComponentBeginOverlap`
  (params (OverlappedComponent :type "PrimitiveComponent Object Reference") (OtherActor :type "Actor Object Reference") (OtherComp :type "PrimitiveComponent Object Reference") (OtherBodyIndex :type Integer) (bFromSweep :type Boolean) (SweepResult :type "HitResult Structure (by ref)"))
  ;[1 1 1] Box1-2 | Comprobación de el cubo que tiene colocado
  (bind _asbp_cubo_puzle (cast `/Game/Blueprints/Caja_Puzle/BP_Cubo_Puzle` OtherActor))
  (bind _tags (`Actor.Tags` _asbp_cubo_puzle))
  (if (and (== (`self.K2_GetActorRotation` _asbp_cubo_puzle) (struct) :`ErrorTolerance` 45.0) (== (`|GetArrayItem` (`ActorComponent.ComponentTags` (`self.Box1-2`))) (`|GetArrayItem` _tags)) (== (`|GetArrayItem` _tags 1) (`|GetArrayItem` (`ActorComponent.ComponentTags` (`self.Box1-2`)) 1)))
    (`KismetSystemLibrary.PrintString` "BIEEN")
    (set `self.booBox1-2` true)
    (`self.K2_SetActorLocation` _asbp_cubo_puzle (`KismetMathLibrary.MakeVector` (`self.row1_X`) (`self.column2_Y`) (`self.zValue`)) false false)
    (`self.AbrirCajon`)
    (else
      (`KismetSystemLibrary.PrintString` "MAAL")
      (set `self.booBox1-2` false))))

(event `self.Box1-3.OnComponentBeginOverlap`
  (params (OverlappedComponent :type "PrimitiveComponent Object Reference") (OtherActor :type "Actor Object Reference") (OtherComp :type "PrimitiveComponent Object Reference") (OtherBodyIndex :type Integer) (bFromSweep :type Boolean) (SweepResult :type "HitResult Structure (by ref)"))
  ;[1 1 1] Box1-3 | Comprobación de el cubo que tiene colocado
  (bind _asbp_cubo_puzle (cast `/Game/Blueprints/Caja_Puzle/BP_Cubo_Puzle` OtherActor))
  (bind _tags (`Actor.Tags` _asbp_cubo_puzle))
  (if (and (== (`self.K2_GetActorRotation` _asbp_cubo_puzle) (struct) :`ErrorTolerance` 45.0) (== (`|GetArrayItem` (`ActorComponent.ComponentTags` (`self.Box1-3`))) (`|GetArrayItem` _tags)) (== (`|GetArrayItem` _tags 1) (`|GetArrayItem` (`ActorComponent.ComponentTags` (`self.Box1-3`)) 1)))
    (`KismetSystemLibrary.PrintString` "BIEEN")
    (set `self.booBox1-3` true)
    (`self.K2_SetActorLocation` _asbp_cubo_puzle (`KismetMathLibrary.MakeVector` (`self.row1_X`) (`self.column3_Y`) (`self.zValue`)) false false)
    (`self.AbrirCajon`)
    (else
      (`KismetSystemLibrary.PrintString` "MAAL")
      (set `self.booBox1-3` false))))

(event `self.Box2-2.OnComponentEndOverlap`
  (params (OverlappedComponent :type "PrimitiveComponent Object Reference") (OtherActor :type "Actor Object Reference") (OtherComp :type "PrimitiveComponent Object Reference") (OtherBodyIndex :type Integer))
  ;[1 1 1] Box2-2 | Comprobación de el cubo que tiene colocado
  (cast `/Game/Blueprints/Caja_Puzle/BP_Cubo_Puzle` OtherActor)
  (set `self.booBox2-2` false))

(event `self.Box2-1.OnComponentEndOverlap`
  (params (OverlappedComponent :type "PrimitiveComponent Object Reference") (OtherActor :type "Actor Object Reference") (OtherComp :type "PrimitiveComponent Object Reference") (OtherBodyIndex :type Integer))
  ;[1 1 1] Box2-1 | Comprobación de el cubo que tiene colocado
  (cast `/Game/Blueprints/Caja_Puzle/BP_Cubo_Puzle` OtherActor)
  (set `self.booBox2-1` false))

(event `self.Box2-3.OnComponentEndOverlap`
  (params (OverlappedComponent :type "PrimitiveComponent Object Reference") (OtherActor :type "Actor Object Reference") (OtherComp :type "PrimitiveComponent Object Reference") (OtherBodyIndex :type Integer))
  ;[1 1 1] Box2-3 | Comprobación de el cubo que tiene colocado
  (cast `/Game/Blueprints/Caja_Puzle/BP_Cubo_Puzle` OtherActor)
  (set `self.booBox2-3` false))

(event `self.Box2-3.OnComponentBeginOverlap`
  (params (OverlappedComponent :type "PrimitiveComponent Object Reference") (OtherActor :type "Actor Object Reference") (OtherComp :type "PrimitiveComponent Object Reference") (OtherBodyIndex :type Integer) (bFromSweep :type Boolean) (SweepResult :type "HitResult Structure (by ref)"))
  ;[1 1 1] Box2-3 | Comprobación de el cubo que tiene colocado
  (bind _asbp_cubo_puzle (cast `/Game/Blueprints/Caja_Puzle/BP_Cubo_Puzle` OtherActor))
  (bind _tags (`Actor.Tags` _asbp_cubo_puzle))
  (if (and (== (`self.K2_GetActorRotation` _asbp_cubo_puzle) (struct) :`ErrorTolerance` 45.0) (== (`|GetArrayItem` (`ActorComponent.ComponentTags` (`self.Box2-3`))) (`|GetArrayItem` _tags)) (== (`|GetArrayItem` _tags 1) (`|GetArrayItem` (`ActorComponent.ComponentTags` (`self.Box2-3`)) 1)))
    (`KismetSystemLibrary.PrintString` "BIEEN")
    (set `self.booBox2-3` true)
    (`self.K2_SetActorLocation` _asbp_cubo_puzle (`KismetMathLibrary.MakeVector` (`self.row2_X`) (`self.column3_Y`) (`self.zValue`)) false false)
    (`self.AbrirCajon`)
    (else
      (`KismetSystemLibrary.PrintString` "MAAL")
      (set `self.booBox2-3` false))))

(event `self.Box2-2.OnComponentBeginOverlap`
  (params (OverlappedComponent :type "PrimitiveComponent Object Reference") (OtherActor :type "Actor Object Reference") (OtherComp :type "PrimitiveComponent Object Reference") (OtherBodyIndex :type Integer) (bFromSweep :type Boolean) (SweepResult :type "HitResult Structure (by ref)"))
  ;[1 1 1] Box2-2 | Comprobación de el cubo que tiene colocado
  (bind _asbp_cubo_puzle (cast `/Game/Blueprints/Caja_Puzle/BP_Cubo_Puzle` OtherActor))
  (bind _tags (`Actor.Tags` _asbp_cubo_puzle))
  (if (and (== (`self.K2_GetActorRotation` _asbp_cubo_puzle) (struct) :`ErrorTolerance` 45.0) (== (`|GetArrayItem` (`ActorComponent.ComponentTags` (`self.Box2-2`))) (`|GetArrayItem` _tags)) (== (`|GetArrayItem` _tags 1) (`|GetArrayItem` (`ActorComponent.ComponentTags` (`self.Box2-2`)) 1)))
    (`KismetSystemLibrary.PrintString` "BIEEN")
    (set `self.booBox2-2` true)
    (`self.K2_SetActorLocation` _asbp_cubo_puzle (`KismetMathLibrary.MakeVector` (`self.row2_X`) (`self.column2_Y`) (`self.zValue`)) false false)
    (`self.AbrirCajon`)
    (else
      (`KismetSystemLibrary.PrintString` "MAAL")
      (set `self.booBox2-2` false))))

(event `self.Box2-1.OnComponentBeginOverlap`
  (params (OverlappedComponent :type "PrimitiveComponent Object Reference") (OtherActor :type "Actor Object Reference") (OtherComp :type "PrimitiveComponent Object Reference") (OtherBodyIndex :type Integer) (bFromSweep :type Boolean) (SweepResult :type "HitResult Structure (by ref)"))
  ;[1 1 1] Box2-1 | Comprobación de el cubo que tiene colocado
  (bind _asbp_cubo_puzle (cast `/Game/Blueprints/Caja_Puzle/BP_Cubo_Puzle` OtherActor))
  (bind _tags (`Actor.Tags` _asbp_cubo_puzle))
  (if (and (== (`self.K2_GetActorRotation` _asbp_cubo_puzle) (struct) :`ErrorTolerance` 45.0) (== (`|GetArrayItem` (`ActorComponent.ComponentTags` (`self.Box2-1`))) (`|GetArrayItem` _tags)) (== (`|GetArrayItem` _tags 1) (`|GetArrayItem` (`ActorComponent.ComponentTags` (`self.Box2-1`)) 1)))
    (`KismetSystemLibrary.PrintString` "BIEEN")
    (set `self.booBox2-1` true)
    (`self.K2_SetActorLocation` _asbp_cubo_puzle (`KismetMathLibrary.MakeVector` (`self.row2_X`) (`self.column1_Y`) (`self.zValue`)) false false)
    (`self.AbrirCajon`)
    (else
      (`KismetSystemLibrary.PrintString` "MAAL")
      (set `self.booBox2-1` false))))

(event `self.Box3-3.OnComponentEndOverlap`
  (params (OverlappedComponent :type "PrimitiveComponent Object Reference") (OtherActor :type "Actor Object Reference") (OtherComp :type "PrimitiveComponent Object Reference") (OtherBodyIndex :type Integer))
  ;[1 1 1] Box3-3 | Comprobación de el cubo que tiene colocado
  (cast `/Game/Blueprints/Caja_Puzle/BP_Cubo_Puzle` OtherActor)
  (set `self.booBox3-3` false))

(event `self.Box3-1.OnComponentEndOverlap`
  (params (OverlappedComponent :type "PrimitiveComponent Object Reference") (OtherActor :type "Actor Object Reference") (OtherComp :type "PrimitiveComponent Object Reference") (OtherBodyIndex :type Integer))
  ;[1 1 1] Box3-1 | Comprobación de el cubo que tiene colocado
  (cast `/Game/Blueprints/Caja_Puzle/BP_Cubo_Puzle` OtherActor)
  (set `self.booBox3-1` false))

(event `self.Box3-2.OnComponentEndOverlap`
  (params (OverlappedComponent :type "PrimitiveComponent Object Reference") (OtherActor :type "Actor Object Reference") (OtherComp :type "PrimitiveComponent Object Reference") (OtherBodyIndex :type Integer))
  ;[1 1 1] Box3-2 | Comprobación de el cubo que tiene colocado
  (cast `/Game/Blueprints/Caja_Puzle/BP_Cubo_Puzle` OtherActor)
  (set `self.booBox3-2` false))

(event `self.Box3-1.OnComponentBeginOverlap`
  (params (OverlappedComponent :type "PrimitiveComponent Object Reference") (OtherActor :type "Actor Object Reference") (OtherComp :type "PrimitiveComponent Object Reference") (OtherBodyIndex :type Integer) (bFromSweep :type Boolean) (SweepResult :type "HitResult Structure (by ref)"))
  ;[1 1 1] Box3-1 | Comprobación de el cubo que tiene colocado
  (bind _asbp_cubo_puzle (cast `/Game/Blueprints/Caja_Puzle/BP_Cubo_Puzle` OtherActor))
  (bind _tags (`Actor.Tags` _asbp_cubo_puzle))
  (if (and (== (`self.K2_GetActorRotation` _asbp_cubo_puzle) (struct) :`ErrorTolerance` 45.0) (== (`|GetArrayItem` (`ActorComponent.ComponentTags` (`self.Box3-1`))) (`|GetArrayItem` _tags)) (== (`|GetArrayItem` _tags 1) (`|GetArrayItem` (`ActorComponent.ComponentTags` (`self.Box3-1`)) 1)))
    (`KismetSystemLibrary.PrintString` "BIEEN")
    (set `self.booBox3-1` true)
    (`self.K2_SetActorLocation` _asbp_cubo_puzle (`KismetMathLibrary.MakeVector` (`self.row3_X`) (`self.column1_Y`) (`self.zValue`)) false false)
    (`self.AbrirCajon`)
    (else
      (`KismetSystemLibrary.PrintString` "MAAL")
      (set `self.booBox3-1` false))))

(event `self.Box3-2.OnComponentBeginOverlap`
  (params (OverlappedComponent :type "PrimitiveComponent Object Reference") (OtherActor :type "Actor Object Reference") (OtherComp :type "PrimitiveComponent Object Reference") (OtherBodyIndex :type Integer) (bFromSweep :type Boolean) (SweepResult :type "HitResult Structure (by ref)"))
  ;[1 1 1] Box3-2 | Comprobación de el cubo que tiene colocado
  (bind _asbp_cubo_puzle (cast `/Game/Blueprints/Caja_Puzle/BP_Cubo_Puzle` OtherActor))
  (bind _tags (`Actor.Tags` _asbp_cubo_puzle))
  (if (and (== (`self.K2_GetActorRotation` _asbp_cubo_puzle) (struct) :`ErrorTolerance` 45.0) (== (`|GetArrayItem` (`ActorComponent.ComponentTags` (`self.Box3-2`))) (`|GetArrayItem` _tags)) (== (`|GetArrayItem` _tags 1) (`|GetArrayItem` (`ActorComponent.ComponentTags` (`self.Box3-2`)) 1)))
    (`KismetSystemLibrary.PrintString` "BIEEN")
    (set `self.booBox3-2` true)
    (`self.K2_SetActorLocation` _asbp_cubo_puzle (`KismetMathLibrary.MakeVector` (`self.row3_X`) (`self.column2_Y`) (`self.zValue`)) false false)
    (`self.AbrirCajon`)
    (else
      (`KismetSystemLibrary.PrintString` "MAAL")
      (set `self.booBox3-2` false))))

(event `self.Box3-3.OnComponentBeginOverlap`
  (params (OverlappedComponent :type "PrimitiveComponent Object Reference") (OtherActor :type "Actor Object Reference") (OtherComp :type "PrimitiveComponent Object Reference") (OtherBodyIndex :type Integer) (bFromSweep :type Boolean) (SweepResult :type "HitResult Structure (by ref)"))
  ;[1 1 1] Box3-3 | Comprobación de el cubo que tiene colocado
  (bind _asbp_cubo_puzle (cast `/Game/Blueprints/Caja_Puzle/BP_Cubo_Puzle` OtherActor))
  (bind _tags (`Actor.Tags` _asbp_cubo_puzle))
  (if (and (== (`self.K2_GetActorRotation` _asbp_cubo_puzle) (struct) :`ErrorTolerance` 45.0) (== (`|GetArrayItem` (`ActorComponent.ComponentTags` (`self.Box3-3`))) (`|GetArrayItem` _tags)) (== (`|GetArrayItem` _tags 1) (`|GetArrayItem` (`ActorComponent.ComponentTags` (`self.Box3-3`)) 1)))
    (`KismetSystemLibrary.PrintString` "BIEEN")
    (set `self.booBox3-3` true)
    (`self.K2_SetActorLocation` _asbp_cubo_puzle (`KismetMathLibrary.MakeVector` (`self.row3_X`) (`self.column3_Y`) (`self.zValue`)) false false)
    (`self.AbrirCajon`)
    (else
      (`KismetSystemLibrary.PrintString` "MAAL")
      (set `self.booBox3-3` false))))

(fn `UserConstructionScript`)