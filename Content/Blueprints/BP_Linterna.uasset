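; BP_Linterna is a grabbable flashlight whose spotlight switches on only while held, through the Encender and Apagar events.
; GrabComponent events track the held state, and dropping it forces the light off.
; A looping timer, started on grab and restarted on drop, writes the spotlight's position, forward vector and on/off state to the LinternaParametros material parameter collection, exposing the beam to materials.
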(event `Encender`
  (bind _spotlight (`self.SpotLight`))
  (if (`self.LinternaCogida`)
    (`SceneComponent.SetVisibility` _spotlight true false)
    (set `self.LinternaLuz` true)
    (else
      (`SceneComponent.SetVisibility` _spotlight false false :!label _label)
      (set `self.LinternaLuz` false))))

(event `Apagar`
  (goto _label))

(event `self.GrabComponent.OnGrabbed`
  (set `self.LinternaCogida` true)
  (`KismetSystemLibrary.K2_SetTimer` null "ComprobacionPosicionLinterna" 0.1 true :!label _label_2))

(event `self.GrabComponent.OnDropped`
  (set `self.LinternaCogida` false)
  (`KismetSystemLibrary.K2_ClearTimer` null "ComprobacionPosicionLinterna")
  (`self.Apagar`)
  (goto _label_2))

(fn `ComprobacionPosicionLinterna`
  (bind _spotlight (`self.SpotLight`))
  (`KismetMaterialLibrary.SetVectorParameterValue` "/Game/VRTemplate/Blueprints/LinternaParametros.LinternaParametros" "PosicionLinterna" (`KismetMathLibrary.Conv_VectorToLinearColor` (`SceneComponent.K2_GetComponentLocation` _spotlight)))
  (`KismetMaterialLibrary.SetVectorParameterValue` "/Game/VRTemplate/Blueprints/LinternaParametros.LinternaParametros" "FordwardVector" (`KismetMathLibrary.Conv_VectorToLinearColor` (`SceneComponent.GetForwardVector` _spotlight)))
  (if (`self.LinternaLuz`)
    (`KismetMaterialLibrary.SetVectorParameterValue` "/Game/VRTemplate/Blueprints/LinternaParametros.LinternaParametros" "Linterna" (make `LinearColor` 1.0 0.0 0.0 1.0))
    (else
      (`KismetMaterialLibrary.SetVectorParameterValue` "/Game/VRTemplate/Blueprints/LinternaParametros.LinternaParametros" "Linterna" (make `LinearColor` 0.0 0.0 0.0 1.0)))))

(fn `UserConstructionScript`)